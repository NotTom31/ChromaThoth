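; BP_Turret is an enemy turret that turns toward the player and shoots at it.
; When PawnSensing sees a BP_AIPlayer, it snaps to face that pawn using only look-at roll and yaw, then spawns an EnemyBullet at its Arrow component after a short delay.
; A Bullet overlapping its Box destroys both the bullet and the turret in a single hit.
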(event OnSeePawn(PawnSensing)
  (params (Pawn :type Pawn%20Object%20Reference))
  (bind _returnvalue (Transformation|GetActorLocation))
  (bind _returnvalue_2 (Transformation|GetActorLocation Pawn))
  (bind _returnvalue_3 (Math|Rotator|FindLookatRotation _returnvalue _returnvalue_2))
  (bind (_roll _pitch _yaw) (Math|Rotator|BreakRotator _returnvalue_3))
  (Utilities|Casting|CastToBP_AIPlayer Pawn)
  (Transformation|SetActorRotation (Math|Rotator|MakeRotator _roll 0.0 _yaw))
  (Utilities|FlowControl|Delay 0.4)
  (Game|SpawnActorfromClass "/Game/Shooting/EnemyBullet.EnemyBullet_C" (Transformation|GetWorldTransform (Variables|Default|GetArrow)) "Undefined" "MultiplyWithRoot" 0 0))

(event OnComponentBeginOverlap(Box)
  (params (OverlappedComponent :type Primitive%20Component%20Object%20Reference) (OtherActor :type Actor%20Object%20Reference) (OtherComp :type Primitive%20Component%20Object%20Reference) (OtherBodyIndex :type Integer) (bFromSweep :type Boolean) (SweepResult :type Hit%20Result%20Structure%20%28by%20ref%29))
  (bind _asbullet (Utilities|Casting|CastToBullet OtherActor))
  (Actor|DestroyActor _asbullet)
  (Actor|DestroyActor))

(event EventBeginPlay)

(event Collision|EventActorBeginOverlap
  (params (OtherActor :type Actor%20Object%20Reference)))

(event EventTick
  (params (DeltaSeconds :type Float%20%28single-precision%29)))

(fn ConstructionScript)