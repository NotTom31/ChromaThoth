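; Bat enemy, shown as a sprite, that homes in on BP_AIPlayer and damages it on contact.
; Tick turns the root toward the player, moves it forward by Velocity at a locked height, and also calls AIMoveTo on the player pawn.
; Box overlap with the player applies DamageOutput and destroys the bat.
; A Bullet hit destroys the bullet, plays a death sound, and only hides the bat and disables its collision.
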(event OnComponentBeginOverlap(Box)
  (params (OverlappedComponent :type Primitive%20Component%20Object%20Reference) (OtherActor :type Actor%20Object%20Reference) (OtherComp :type Primitive%20Component%20Object%20Reference) (OtherBodyIndex :type Integer) (bFromSweep :type Boolean) (SweepResult :type Hit%20Result%20Structure%20%28by%20ref%29))
  (bind _asbp_aiplayer (Utilities|Casting|CastToBP_AIPlayer OtherActor)
    (:then
      (Game|Damage|ApplyDamage _asbp_aiplayer (Variables|Default|GetDamage%20Output) 0 0)
      (Actor|DestroyActor))
    (:CastFailed
      (bind _asbullet (Utilities|Casting|CastToBullet OtherActor))
      (Actor|DestroyActor _asbullet)
      (Rendering|SetVisibility (Variables|Default|Getbat_enemy_Sprite) false false)
      (Collision|SetCollisionEnabled (Variables|Default|GetBox) "NoCollision")
      (Audio|PlaySound2D "/Game/Audio/Death_minor.Death_minor" 1.0 1.0 0.0 0 0))))

(event EventBeginPlay)

(event Collision|EventActorBeginOverlap
  (params (OtherActor :type Actor%20Object%20Reference)))

(event EventTick
  (params (DeltaSeconds :type Float%20%28single-precision%29))
  (bind _returnvalue (Transformation|GetActorLocation))
  (bind (_x _y) (Math|Vector|BreakVector _returnvalue))
  (bind _returnvalue_2 (Actor|GetActorOfClass "/Game/GridMovement/BP_AIPlayer.BP_AIPlayer_C"))
  (Transformation|SetWorldRotation (Variables|Default|GetDefaultSceneRoot) (Math|Rotator|FindLookatRotation (Transformation|GetActorLocation) (Transformation|GetActorLocation _returnvalue_2)) false false)
  (Transformation|AddActorLocalOffset (* (* DeltaSeconds (Variables|Default|GetVelocity)) (Transformation|GetActorForwardVector)) false false)
  (Transformation|SetActorLocation (Math|Vector|MakeVector _x _y 1e+02) false false)
  (AI|AIMoveTo 0 "0, 0, 0" (Game|Player|GetPlayerPawn 0) 5.0 false))

(fn ConstructionScript)