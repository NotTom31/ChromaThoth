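; Wave spawner for bat enemies, spawning Bat_BP just above randomly picked Ground_SpawnEnemy actors gathered at BeginPlay.
; SpawnEnemy is bound to TileMovement_GM's next-wave event and loops over the current wave's count, with a random Delay inside the loop.
; After the loop, WaveIncrement selects the next of four wave counts and prints as debug, or spawns Nosferatu once the fourth wave is reached.
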(event Custom|Spawn%20Enemy
  (bind _wallarray (Variables|Default|GetWallArray))
  (bind _wallarray_2 (Variables|Default|GetWallArray))
  ;[1 1 1] Wave Logic
  (for _index (range 0 (- (Variables|Default|GetEnemySpawnAmount) 1))
    (Utilities|FlowControl|Delay (Math|Random|RandomFloatinRange 0.0 (Variables|Default|GetMax%20Spawn%20Time)))
    ;[1 1 1] Spawn Logic
    (bind _returnvalue (Actor|GetActorOfClass "/Game/GridMovement/BP_AIPlayer.BP_AIPlayer_C"))
    (Game|SpawnActorfromClass "/Game/Enemies/Bat_BP.Bat_BP_C" (Math|Transform|MakeTransform (+ "0.000000,0.000000,10.000000" (Transformation|GetActorLocation (Utilities|Array|Get(acopy) _wallarray (Math|Random|RandomInteger (Utilities|Array|Length _wallarray))))) "0, 0, 0" "0.250000,0.250000,0.250000") "AlwaysSpawn" "MultiplyWithRoot" 0 0))
  (switch int (Variables|Default|GetWaveIncrement)
    (:0
      (Variables|Default|SetEnemySpawnAmount (Variables|Default|GetWave2EnemyCount))
      (bind _result (Math|Integer|IncrementInt (Variables|Default|GetWaveIncrement) :!label _label)
        (:%20%20
          (Development|PrintString (Utilities|String|ToString(Integer) _result) true true "(R=1.000000,G=0.000000,B=0.136188,A=1.000000)"))))
    (:1
      (Variables|Default|SetEnemySpawnAmount (Variables|Default|GetWave3EnemyCount))
      (goto _label))
    (:2
      (Variables|Default|SetEnemySpawnAmount (Variables|Default|GetWave4EnemyCount))
      (goto _label))
    (:3
      (Game|SpawnActorfromClass "/Game/Enemies/Nosferatu.Nosferatu_C" (Math|Transform|MakeTransform (Transformation|GetActorLocation (Utilities|Array|Get(acopy) _wallarray_2 (Math|Random|RandomInteger (Utilities|Array|Length _wallarray_2)))) "0, 0, 0" "0.250000,0.250000,0.250000") "Undefined" "MultiplyWithRoot" 0 0))))

(event EventBeginPlay
  ;[1 1 1] Wave Logic
  (Variables|Default|SetEnemySpawnAmount (Variables|Default|GetWave1EnemyCount))
  (bind _outactors (Actor|GetAllActorsOfClass "/Game/GridMovement/Ground_SpawnEnemy.Ground_SpawnEnemy_C"))
  (Variables|Default|SetWallArray _outactors)
  (bind _astile_movement_gm (Utilities|Casting|CastToTileMovement_GM (Game|GetGameMode)))
  (EventDispatchers|BindEventtoSpawnNextWave _astile_movement_gm (delegate Custom|Spawn%20Enemy)))

(event Collision|EventActorBeginOverlap
  (params (OtherActor :type Actor%20Object%20Reference))
  ;[1 1 1] Spawn Logic
)

(event EventTick
  (params (DeltaSeconds :type Float%20%28single-precision%29))
  ;[1 1 1] Spawn Logic
)

(fn ConstructionScript)