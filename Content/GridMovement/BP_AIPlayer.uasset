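; BP_AIPlayer is a paper-sprite AI pawn that chases the player and carries the health whose loss ends the game.
; Tick reissues AI MoveTo toward the player pawn and flips the sprite by Y velocity, while BeginPlay registers it on PlayerPawn.
; Damage triggers sound, camera shake and a damage widget, or at zero health pauses into the game-over screen.
; SetCoord stores the player's truncated location as a target tile.
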(event Custom|Apply%20Damage
  (params (Damage :type Float%20%28double-precision%29))
  (Game|Damage|ApplyDamage self Damage 0 0))

(event EventBeginPlay
  (bind _asplayer_pawn (Utilities|Casting|CastToPlayerPawn (Game|Player|GetPlayerPawn 0)))
  (Variables|/Game/GridMovement/PlayerPawn.PlayerPawn_C|SetAI_Player _asplayer_pawn self)
  (Game|SetGamePaused false))

(event EventTick
  (params (DeltaSeconds :type Float%20%28single-precision%29))
  (bind _papersprite (Variables|Default|GetPaperSprite))
  (AI|AIMoveTo self (Transformation|GetActorLocation (Game|Player|GetPlayerPawn 0)) 0 0.0 false
    (:then
      (if (> (.Y (Math|Vector|BreakVector (Variables|/Script/Engine.MovementComponent|GetVelocity (Variables|Character|GetCharacterMovement)))) 0.0)
        (Transformation|SetRelativeScale3D _papersprite "-0.080000,1.000000,0.080000")
        (else
          (Transformation|SetRelativeScale3D _papersprite "0.080000,1.000000,0.080000"))))))

(event Game|Damage|EventAnyDamage
  (params (Damage :type Float%20%28single-precision%29) (DamageType :type Damage%20Type%20Object%20Reference) (InstigatedBy :type Controller%20Object%20Reference) (DamageCauser :type Actor%20Object%20Reference))
  (bind _returnvalue (Game|GetPlayerController 0))
  (if (not (Variables|Default|GetIsDead))
    (Variables|Default|SetHealth (- (Variables|Default|GetHealth) Damage))
    (if (<= (Variables|Default|GetHealth) 0.0)
      (Variables|Default|SetIsDead true)
      (Audio|PlaySound2D "/Game/Audio/Death_1.Death_1" 1.0 1.0 0.0 0 0)
      (bind _returnvalue_2 (UserInterface|CreateWidget "/Game/Widgets/WB_GameOver.WB_GameOver_C" (Game|GetPlayerController 0)))
      (UserInterface|Viewport|AddtoViewport _returnvalue_2 0)
      (Variables|/Script/Engine.PlayerController|SetbShowMouseCursor _returnvalue true)
      (Input|SetInputModeUIOnly _returnvalue _returnvalue_2 "DoNotLock" false)
      (Game|SetGamePaused true)
      (else
        (Development|PrintString (Utilities|String|ToString(Float) (Variables|Default|GetHealth)))
        (Audio|PlaySound2D 0 1.0 1.0 0.0 0 0)
        (Camera|PlayWorldCameraShake "/Game/Camera/CameraShake_BP.CameraShake_BP_C" "0, 0, 0" 0.0 1e+05)
        (bind _returnvalue_3 (UserInterface|CreateWidget "/Game/Widgets/WB_Damage.WB_Damage_C" (Game|GetPlayerController 0)))
        (UserInterface|Viewport|AddtoViewport _returnvalue_3 0)))))

(fn ConstructionScript)

(fn GetCoord)

(fn SetCoord
  (bind _returnvalue (Game|Player|GetPlayerPawn 0))
  (bind _returnvalue_2 (Transformation|GetActorLocation _returnvalue))
  (Variables|Default|SetTile%20to%20Move%20To (Utilities|Struct|MakeCoord (Math|Float|Truncate (.x _returnvalue_2)) (Math|Float|Truncate (.y _returnvalue_2))))
  (Development|PrintString "Set coord"))