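; Axe head item for the point-and-click ForestDemo scene that combines with a stick handle to form an axe.
; Receiving the Stick Handle deactivates the axe head, activates the referenced axe item, plays dialogue and reports the item as consumed.
; Any other item plays an invalid-use dialogue and is rejected.
; Pickup makes the character look at the axe head and plays a dialogue, then returns false.
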(fn ConstructionScript
  (|CallParentFunction))

(fn RecieveItem
  (params (ItemName :type Name :default "None"))
  (switch name ItemName
    (:Default
      (CallFunction|StartDialogueSequence "InvalidRecieveItem")
      (return false false))
    (:StickHandle
      (CallFunction|SetItemActiveState false)
      (Default|SetItemActiveState (Variables|System|GetAxeItem) true)
      (CallFunction|StartDialogueSequence "RecieveItemAxeHead")
      (return true true))))

(fn Pickup
  (params (Instigator :type Actor%20Object%20Reference))
  (Class|BPICharacter|Lookat(Message) (CallFunction|GetPNCCharacter) (Transformation|GetActorLocation))
  (CallFunction|StartDialogueSequence "PickupAxehead")
  (return false))