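; BP_Item_Hat is a pickup item in the PNC ForestDemo scene that puts a hat on the player character instead of going into the inventory.
; A successful parent Pickup calls AddHatToCharacter, which creates a static mesh component at runtime and attaches it to the character mesh's head socket with a relative offset.
; BeginPlay re-adds the hat when the item is inactive, restoring it for saved games.
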(event EventBeginPlay
  ;[1 1 1] If the game is saved and the item is inactive, then add the hat to the player.
  (if (not (Variables|Default|GetbIsActive))
    (CallFunction|AddHattoCharacter)))

(fn ConstructionScript
  (|CallParentFunction))

(fn IsInventoryItem
  (return false))

(fn Pickup
  (params (Instigator :type Actor%20Object%20Reference))
  (bind _success (|CallParentFunction Instigator))
  (if _success
    (CallFunction|AddHattoCharacter))
  (return _success))

(fn AddHattoCharacter
  (bind _returnvalue (AddComponent|AddStaticMeshComponent (CallFunction|GetPNCCharacter) true (Math|Transform|MakeTransform "10.000000,2.000000, 0" "-90.000000, 0, 0" "1,1,1")))
  (Components|StaticMesh|SetStaticMesh _returnvalue "/Game/PNCTookit/PNCGame/Scenes/ForestDemo/SceneContent/Meshes/SM_Hat.SM_Hat")
  (Rendering|SetReceivesDecals _returnvalue false)
  (Transformation|AttachComponentToComponent _returnvalue (Variables|/Script/Engine.Character|GetMesh (CallFunction|GetPNCCharacter)) "head" "KeepRelative" "KeepRelative" "KeepRelative" true))