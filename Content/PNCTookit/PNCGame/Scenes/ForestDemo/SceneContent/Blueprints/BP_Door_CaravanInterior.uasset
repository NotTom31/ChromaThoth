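; Caravan interior door for the ForestDemo scene that plays a one-time shop intro dialogue.
; It overrides StartDoorDialogue: for one specific arrived location, it checks the Scene Manager's state strings for SceneIntro.
; When present, it removes that state, starts the ShopSceneIntro dialogue sequence and returns true.
; All other cases fall back to the parent door's dialogue logic.
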(event EventBeginPlay
  (|CallParentFunction) ; This node is disabled and will not be called.\nDrag off pins to build functionality.
)

(event Collision|EventActorBeginOverlap
  (params (OtherActor :type Actor%20Object%20Reference)))

(event EventTick
  (params (DeltaSeconds :type Float%20%28single-precision%29)))

(fn ConstructionScript
  (|CallParentFunction))

(fn StartDoorDialogue
  (params (ArrivedLocation :type EDoorLocation%20Enum :default "NewEnumerator2"))
  (if (Utilities|Enum|Equal(Enum) ArrivedLocation "NewEnumerator0")
    (if (Utilities|Array|ContainsItem (Default|GetStateStrings (CallFunction|GetSceneManager)) "SceneIntro")
      (Default|RemoveStateStringfromScene (CallFunction|GetSceneManager) "" "SceneIntro")
      (CallFunction|StartDialogueSequence "ShopSceneIntro")
      (return true)
      (else
        _)))
  (bind _return (|CallParentFunction ArrivedLocation))
  (return _return))