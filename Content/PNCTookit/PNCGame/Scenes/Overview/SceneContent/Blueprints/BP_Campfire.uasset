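; Interactable campfire for a point-and-click game that lights when given chopped wood and shows different inspection dialogue when lit or unlit.
; Accepted wood is stored in its inventory component, then SetBonfireState toggles the fire particle, point light and wood mesh, and activation dialogue plays.
; A timeline scales the light's starting intensity for flicker.
; On state load, stored wood sets the fire to inactive.
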(event EventBeginPlay
  ;[1 0.8888 0.4989 0.3] Animate a flicker effect for the fire light
  (Variables|Default|SetLightIntensity (Variables|/Script/Engine.LightComponentBase|GetIntensity (Variables|Components|GetFirePointLight)))
  (bind _brightness (Timeline|FireBrightness Play)
    (:Update
      (Rendering|Components|Light|SetIntensity (Variables|Components|GetFirePointLight) (* (Variables|Default|GetLightIntensity) _brightness)))))

(fn ConstructionScript
  (|CallParentFunction))

(fn OnInspection
  (params (Inspector :type Controller%20Object%20Reference))
  (if (Variables|Default|GetbIsActive)
    (CallFunction|StartDialogueSequence "InspectCampfireLit" Inspector)
    (else
      (CallFunction|StartDialogueSequence "InspectCampfireUnlit" Inspector)))
  (return true))

(fn SetBonfireState
  (params (Active :type Boolean))
  (bind _output_get (Variables|Default|SetbIsActive Active))
  (if _output_get
    (Components|Activation|Activate (Variables|Components|GetFireParticle) true)
    (Rendering|SetVisibility (Variables|Components|GetFirePointLight) true false)
    (else
      (Components|Activation|Deactivate (Variables|Components|GetFireParticle))
      (Rendering|SetVisibility (Variables|Components|GetFirePointLight) false false))))

(fn LoadGameplayState
  (if (Default|HasIteminInventory (Variables|Components|GetBP_InventoryComponent) "ChoppedWood")
    (CallFunction|SetBonfireState false))
  (return true))

(fn GetItemName
  (return "None"))

(fn IsInventoryItem
  (return false))

(fn Pickup
  (params (Instigator :type Actor%20Object%20Reference))
  (return false))

(fn RecieveItem
  (params (ItemName :type Name :default "None"))
  (switch name ItemName
    (:Default
      (return false false))
    (:ChoppedWood
      (bind _return (Default|AddInventoryItem (Variables|Components|GetBP_InventoryComponent) "ChoppedWood"))
      (CallFunction|SetBonfireState _return)
      (if _return
        (CallFunction|StartDialogueSequence "ActiveCampfire"))
      (return _return _return))))