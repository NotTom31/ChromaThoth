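; BP_Clock is an interactable scene clock for a point-and-click game that tells the real time once it has been used.
; The first successful use sets IsUsed; each use plays a state-dependent dialogue.
; Inspection plays dialogue until used, then shows the current time in a single floating widget, removed after a short delay.
; Pickup is refused with dialogue, while received items are accepted and consumed with a storage dialogue.
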(event Custom|DelayRemoveFloatingDialogue
  (Utilities|FlowControl|Delay 3.0)
  (Widget|RemovefromParent (Variables|Default|GetFloatingDialogueRef))
  (Variables|Default|SetFloatingDialogueRef 0))

(fn ConstructionScript
  (|CallParentFunction))

(fn UseObject
  (params (InteractingCharacter :type BP%20PNC%20Character%20Parent%20Object%20Reference))
  (bind _success (|CallParentFunction InteractingCharacter))
  (if _success
    (if (Variables|Default|GetbIsUsed)
      (CallFunction|StartDialogueSequence "UseClockOn" self)
      (else
        (Variables|Default|SetbIsUsed true)
        (CallFunction|StartDialogueSequence "UseClockOff" self))))
  (return _success))

(fn DisplayTimeDialogue
  (Variables|Default|GetFloatingDialogueRef
    (:then)
    (:else
      (bind _returnvalue (UserInterface|CreateWidget "/Game/PNCTookit/Blueprints/Gameplay/Dialogue/Widgets/WBP_FloatingDialogueText.WBP_FloatingDialogueText_C" 0 self 0 (Utilities|Struct|MakeSDialogueData (Utilities|Array|MakeArray "") (Utilities|Text|FormatText "The time is {time}" (Class|KismetTextLibrary|AsTimeDateTime (Math|DateTime|Now))) (Utilities|Array|MakeArray "") "(SpeakersName_25_3506AB8C447AA4DC59B2849A601E9572=\"\",CharacterTag_26_9B5F60264BAC99304CFD3084E91243E5=(TagName=\"Character.Player\"),CharacterImage_3_C4EA34A34D2E4556D1C156A2FEAB0F83=None,CharacterAnimation_7_E8268226472B2FDC816594B058214AB0=NewEnumerator8,TextColour_11_75E7AA0F4B1CBE19D1145F94D001491C=(R=1.000000,G=1.000000,B=1.000000,A=1.000000),DurationOverride_14_CCB259D7454D4C5E2D4B10B57696C999=2.000000,DisplayType_21_0DD9926E4FC4D6E85D023099A0AA7E78=NewEnumerator1)" "(SoundWave_9_A24262394181C4100E217997FEA3103E=None,DialogueWave_2_339C59A344308554C3D695A557BA9116=None,Context_5_AE4828A94E29B7BE32F9A6864A54A7FC=(Speaker=None,Targets=(None)))")))
      (bind _output_get (Variables|Default|SetFloatingDialogueRef _returnvalue))
      (UserInterface|Viewport|AddtoViewport _output_get 0)
      (CallFunction|DelayRemoveFloatingDialogue))))

(fn OnInspection
  (params (Inspector :type Controller%20Object%20Reference))
  (if (Variables|Default|GetbIsUsed)
    (CallFunction|DisplayTimeDialogue)
    (return true)
    (else
      (CallFunction|StartDialogueSequence "InspectClock" self)
      (return true))))

(fn GetItemName
  (return "None"))

(fn IsInventoryItem
  (return false))

(fn Pickup
  (params (Instigator :type Actor%20Object%20Reference))
  (CallFunction|StartDialogueSequence "PickupClockToHeavy" self)
  (return false))

(fn RecieveItem
  (params (ItemName :type Name :default "None"))
  (CallFunction|StartDialogueSequence "RecieveItemClockStorage" self)
  (return true true))