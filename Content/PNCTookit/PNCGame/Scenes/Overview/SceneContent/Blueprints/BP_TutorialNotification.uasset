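; BP_TutorialNotification is an actor for the Overview scene that displays a tutorial text notification through its widget component.
; On BeginPlay it creates a WBP_TutorialText widget from its TutorialText, assigns it to the component and sets visibility from IsEnabled.
; EnableTutorialNotification updates IsEnabled and shows or hides the component to match.
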(event EventBeginPlay
  (bind _returnvalue (UserInterface|CreateWidget "/Game/PNCTookit/PNCGame/Scenes/Overview/SceneContent/Blueprints/WBP_TutorialText.WBP_TutorialText_C" 0 self (Variables|Default|GetTutorialText)))
  (UserInterface|SetWidget (Variables|Default|GetWidget) _returnvalue)
  (Rendering|SetVisibility (Variables|Default|GetWidget) (Variables|Default|GetbIsEnabled) false))

(fn ConstructionScript)

(fn EnableTutorialNotification
  (params (Enable :type Boolean))
  (bind _output_get (Variables|Default|SetbIsEnabled Enable))
  (Rendering|SetVisibility (Variables|Default|GetWidget) _output_get false))