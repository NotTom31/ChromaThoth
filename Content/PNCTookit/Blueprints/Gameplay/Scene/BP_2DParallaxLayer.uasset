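; BP_2DParallaxLayer is a scene layer actor that shifts horizontally to create 2D parallax.
; Its construction script snaps each valid actor in ParalaxChildren to the layer's Z and attaches it, keeping world transforms.
; It stores its location on BeginPlay; SetParallaxOffset then sets X to initial X plus Offset, with that whole sum scaled by ParalaxMultiplyer, keeping initial Y and Z.
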(event Custom|SetParallaxOffset
  (params (Offset :type Float%20%28single-precision%29))
  (bind _initiallocation (Variables|Default|GetInitialLocation))
  ;[1 0.6542 0.2113 0.3] Set Parallax
  (bind _output_get (Variables|Default|SetGoalLocation (Math|Vector|MakeVector (* (+ (.x _initiallocation) Offset) (Variables|Default|GetParalaxMultiplyer)) (.y _initiallocation) (.z _initiallocation))))
  (Transformation|SetActorLocation _output_get false false))

(event EventBeginPlay
  ;[1 0.6542 0.2113 0.3] Set actors initial location
  (Variables|Default|SetInitialLocation (Transformation|GetActorLocation)))

(fn ConstructionScript
  (for _array_element (Variables|Default|GetParalaxChildren)
    (Utilities|IsValid _array_element
      (:Is%20Valid
        (Transformation|SetActorLocation _array_element (Math|Vector|MakeVector (.x (Transformation|GetActorLocation _array_element)) (.y (Transformation|GetActorLocation _array_element)) (.z (Transformation|GetActorLocation self))) false false)
        (Transformation|AttachActorToActor _array_element self "None" "KeepWorld" "KeepWorld" "KeepWorld" true)))))