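; Scene manager that maps interactable actors to their BP_InteractionVolume, with lookup, override and debug display toggling.
; After load completes, it caches every placed volume in an array and maps each assigned actor to that volume's index.
; Interactable objects, items and doors left without a volume can opt in, via BP_GlobalInteractionComponent, to one spawned at the closest nav point and rotated toward the actor.
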(event EventBeginPlay
  ;[0.8347 0.5698 1 0.3] Cache all found interaction volumes and their associated actors
  (Utilities|IsLoadComplete
    (:Load%20Complete
      (bind _outactors (Actor|GetAllActorsOfClass "/Game/PNCTookit/Blueprints/Gameplay/Scene/BP_InteractionVolume.BP_InteractionVolume_C"))
      (for _array_element _outactors
        (CallFunction|AddInteractionVolume _array_element))
      (CallFunction|FindMissingActorVolumes))))

(fn ConstructionScript)

(fn AddInteractionVolume
  (params (InteractionVolume :type BP%20Interaction%20Volume%20Object%20Reference))
  ;[1 0.3458 0.2661 0.3] Add the interaction volume to the volumes array and set the index for the actor
  (Utilities|IsValid InteractionVolume
    (:Is%20Valid
      (if (not (Utilities|Array|ContainsItem (Variables|System|GetInteractionVolumeArray) InteractionVolume))
        (Utilities|Array|AddUnique (Variables|System|GetInteractionVolumeArray) InteractionVolume)
        (for _array_element (Variables|/Game/PNCTookit/Blueprints/Gameplay/Scene/BP_InteractionVolume.BP_InteractionVolume_C|GetAssignedActorsRef InteractionVolume)
          (if (not (.ReturnValue (Utilities|Map|Find (Variables|System|GetActorList) _array_element)))
            (Utilities|Map|Add (Variables|System|GetActorList) _array_element (Utilities|Array|FindItem (Variables|System|GetInteractionVolumeArray) InteractionVolume))))))))

(fn GetActorsInteractionVolume
  (params (Actor :type Actor%20Object%20Reference))
  (bind _actorlist (Variables|System|GetActorList))
  (bind (_value _returnvalue) (Utilities|Map|Find _actorlist Actor))
  ;[0.4906 1 0.4549 0.3] Return a reference to the given actors  interaction volume
  (Utilities|IsValid Actor
    (:Is%20Valid
      (if _returnvalue ; Was the actor found?
        (return (Utilities|Array|Get(acopy) (Variables|System|GetInteractionVolumeArray) _value))
        (else
          _)))
    (:Is%20Not%20Valid
      _))
  (return 0))

(fn OverrideInteractionVolume
  (params (Actor :type Actor%20Object%20Reference) (InteractionVolume :type BP%20Interaction%20Volume%20Object%20Reference))
  ;[1 0.9111 0.3623 0.3] Override the interaction volume for the given actor
  (if (.ReturnValue (Utilities|Map|Find (Variables|System|GetActorList) Actor)) ; Does the actor exist, and already have an interaction volume assigned?
    (Utilities|Map|Add (Variables|System|GetActorList) Actor (Utilities|Array|FindItem (Variables|System|GetInteractionVolumeArray) InteractionVolume))
    (else
      (Utilities|Array|AddUnique (Variables|/Game/PNCTookit/Blueprints/Gameplay/Scene/BP_InteractionVolume.BP_InteractionVolume_C|GetAssignedActorsRef InteractionVolume) Actor)
      (CallFunction|AddInteractionVolume InteractionVolume))))

(fn FindMissingActorVolumes
  ;[1 0.7077 0.2831 0.3] Find interactable objects with missing interaction volumes. Loop through all the actors and spawn a new volume (if enabled on the actor)
  (bind _outactors (Actor|GetAllActorsOfClass "/Game/PNCTookit/Blueprints/Gameplay/Scene/BP_InteractableObjectBase.BP_InteractableObjectBase_C"))
  (Utilities|Array|AppendArray (LocalVariables|GetActorArray) _outactors)
  (bind _outactors_2 (Actor|GetAllActorsOfClass "/Game/PNCTookit/Blueprints/Gameplay/Items/BP_ItemBase.BP_ItemBase_C"))
  (Utilities|Array|AppendArray (LocalVariables|GetActorArray) _outactors_2)
  (bind _outactors_3 (Actor|GetAllActorsOfClass "/Game/PNCTookit/Blueprints/Gameplay/Scene/BP_DoorBase.BP_DoorBase_C"))
  (Utilities|Array|AppendArray (LocalVariables|GetActorArray) _outactors_3)
  (for _array_element (LocalVariables|GetActorArray)
    (if (not (.ReturnValue (Utilities|Map|Find (Variables|System|GetActorList) _array_element)))
      (if (Variables|/Game/PNCTookit/Blueprints/Components/BP_GlobalInteractionComponent.BP_GlobalInteractionComponent_C|GetbSpawnMissingInteractionVolume (Actor|GetComponentbyClass _array_element "/Game/PNCTookit/Blueprints/Components/BP_GlobalInteractionComponent.BP_GlobalInteractionComponent_C")) ; Should the manager spawn a missing interaction \nvolume for the actor?
        (bind _returnvalue (Game|SpawnActorfromClass "/Game/PNCTookit/Blueprints/Gameplay/Scene/BP_InteractionVolume.BP_InteractionVolume_C" (Math|Conversions|ToTransform(Vector) (.NavLocation (CallFunction|GetClosestNavPointatLocation (Transformation|GetActorLocation _array_element)))) "Undefined" 0 0))
        (Utilities|Array|AddUnique (Variables|/Game/PNCTookit/Blueprints/Gameplay/Scene/BP_InteractionVolume.BP_InteractionVolume_C|GetAssignedActorsRef _returnvalue) _array_element)
        (CallFunction|AddInteractionVolume _returnvalue)
        (Transformation|SetActorRotation _returnvalue (Math|Rotator|MakeRotator (.roll (Math|Rotator|CombineRotators (Math|Rotator|FindLookatRotation (Transformation|GetActorLocation _returnvalue) (Transformation|GetActorLocation _array_element)) "0,90.000000, 0")) 0.0 (.yaw (Math|Rotator|CombineRotators (Math|Rotator|FindLookatRotation (Transformation|GetActorLocation _returnvalue) (Transformation|GetActorLocation _array_element)) "0,90.000000, 0"))))
        (CallFunction|CustomPrint (Utilities|String|Append "Found Interactable Object \" " (Utilities|GetDisplayName _array_element) " \" without an interaction volume. Adding Interaction Volume for the actor.") "NewEnumerator0" false)
        (CallFunction|CustomPrint "Tip: Generated Interaction Volumes can still result in strange behavior. Add your own volume for interactable actors in your scene for a better result. " "NewEnumerator0" false)))))

(fn EnableVolumeDebug
  (params (Debug%20Enabled :type Boolean))
  ;[1 0.5909 0.2499 0.3] Show / Hide all interaction volumes visability in game. Also displays whether the character is overlapping the volume
  (if (Math|Boolean|NotEqual(Boolean) Debug%20Enabled (Variables|Settings|GetbEnableDebug))
    (Variables|Settings|SetbEnableDebug Debug%20Enabled)
    (bind _outactors (Actor|GetAllActorsOfClass "/Game/PNCTookit/Blueprints/Gameplay/Scene/BP_InteractionVolume.BP_InteractionVolume_C"))
    (for _array_element _outactors
      (Default|EnableDebug _array_element (Variables|Settings|GetbEnableDebug)))))