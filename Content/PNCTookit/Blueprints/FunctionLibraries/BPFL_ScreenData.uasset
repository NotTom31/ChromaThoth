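; Blueprint function library of screen-space helpers for keeping UI widgets inside the viewport.
; The mouse and screen-position functions clamp a point to viewport bounds using widget size and global and per-axis edge offsets, with the latter centering the widget horizontally above the point.
; A third function reports whether a screen position lies on or beyond the viewport edge and returns which side, checking horizontal edges before vertical.
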(fn GetMousePositioninRange
  (params (WidgetSizeOffset :type Vector%202D%20Structure) (GlobalEdgeOffset :type Float%20%28double-precision%29) (XEdgeOffset :type Float%20%28double-precision%29) (YEdgeOffset :type Float%20%28double-precision%29))
  (bind (_x _y) (Math|Vector2D|BreakVector2D WidgetSizeOffset))
  (bind _returnvalue (Game|GetPlayerController 0))
  (bind _returnvalue_2 (Viewport|GetViewportSize))
  (bind _returnvalue_3 (Math|Float|MakeLiteralFloat GlobalEdgeOffset))
  (bind (_locationx _locationy) (Game|Player|GetMousePosition _returnvalue))
  (bind (_x_2 _y_2) (Math|Vector2D|BreakVector2D _returnvalue_2))
  (return (CallFunction|ClampVector2D (Math|Vector2D|MakeVector2D (Math|Float|Clamp(Float) _locationx _x (- (- _x_2 _returnvalue_3) (+ _x XEdgeOffset))) (- (Math|Float|Clamp(Float) _locationy _y (- (- _y_2 _returnvalue_3) (- _y YEdgeOffset))) YEdgeOffset)) "(X=0.100000,Y=0.100000)" (- (Viewport|GetViewportSize) 0.1))))

(fn GetScreenPositioninRange
  (params (WidgetSize :type Vector%202D%20Structure) (ScreenPos :type Vector%202D%20Structure) (GlobalEdgeOffset :type Float%20%28double-precision%29) (XEdgeOffset :type Float%20%28double-precision%29) (YEdgeOffset :type Float%20%28double-precision%29))
  (bind _y (Math|Vector2D|BreakVector2D WidgetSize))
  (bind _x (Math|Vector2D|BreakVector2D WidgetSize))
  (return (CallFunction|ClampVector2D (Math|Vector2D|MakeVector2D (Math|Float|Clamp(Float) (- (.X (Math|Vector2D|BreakVector2D ScreenPos)) (/ _x 2.0)) (+ GlobalEdgeOffset XEdgeOffset) (- (- (- (.X (Math|Vector2D|BreakVector2D (Viewport|GetViewportSize))) _x) GlobalEdgeOffset) XEdgeOffset)) (Math|Float|Clamp(Float) (- (.Y (Math|Vector2D|BreakVector2D ScreenPos)) _y) (+ GlobalEdgeOffset YEdgeOffset) (- (- (- (.Y (Math|Vector2D|BreakVector2D (Viewport|GetViewportSize))) _y) GlobalEdgeOffset) YEdgeOffset))) "(X=0.100000,Y=0.100000)" (- (Viewport|GetViewportSize) 0.1))))

(fn GetScreenOutOfRangeDirection
  (params (ScreenPos :type Vector%202D%20Structure))
  (bind _returnvalue (Viewport|GetViewportSize))
  (bind (_x _y) (Math|Vector2D|BreakVector2D ScreenPos))
  (bind (_x_2 _y_2) (Math|Vector2D|BreakVector2D _returnvalue))
  ;[0.4247 0.6963 1 0.3] If the screen position is out of the visible screens bounds, return the screen direction
  (if (<= _x 0.0)
    (LocalVariables|SetDirection "NewEnumerator2")
    (elif (>= _x _x_2)
      (LocalVariables|SetDirection "NewEnumerator3")
      (elif (<= _y 0.0)
        (LocalVariables|SetDirection "NewEnumerator0")
        (elif (>= _y _y_2)
          (LocalVariables|SetDirection "NewEnumerator1")
          (else
            (return false "NewEnumerator0"))))))
  (return true (LocalVariables|GetDirection)))