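; Miscellaneous Blueprint function library in the PNCTookit folder, providing small helpers for mouse projection, target search, viewport scale and coordinate conversion.
; It deprojects the mouse to a world point at a given distance and loops through actors to pick the location closest to a start point.
; The viewport scale getter passes through GetViewportScale unchanged.
; Relative-to-world conversion only adds the actor's location, ignoring rotation and scale.
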(fn MousetoWorldPosition
  (params (PlayerController :type Player%20Controller%20Object%20Reference) (Distance :type Float%20%28single-precision%29))
  (bind (_worldlocation _worlddirection) (Game|Player|ConvertMouseLocationToWorldSpace PlayerController))
  (return (+ _worldlocation (* _worlddirection Distance))))

(fn FindClosestTargetLocationinArray
  (params (StartLocation :type Vector) (ToLocations :type Array%20of%20Target%20Point%20Object%20References))
  (for _array_element ToLocations
    (if (< (Math|Vector|VectorLength (- (Transformation|GetActorLocation _array_element) StartLocation)) (LocalVariables|GetClosestVectorDistance))
      (LocalVariables|SetClosestVectorDistance (Math|Vector|VectorLength (- (Transformation|GetActorLocation _array_element) StartLocation)))
      (LocalVariables|SetClosestVector (Transformation|GetActorLocation _array_element))))
  (return (LocalVariables|GetClosestVector)))

(fn GetViewportScaleModifiable
  (return (Class|WidgetLayoutLibrary|GetViewportScale)))

(fn ConvertRelativeVectortoWorld
  (params (RelativeVector :type Vector) (Actor :type Actor%20Object%20Reference))
  (return (+ RelativeVector (Transformation|GetActorLocation Actor))))