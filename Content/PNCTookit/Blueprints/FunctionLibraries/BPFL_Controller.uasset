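; Blueprint function library of global shortcuts to the PNC toolkit's core player objects: character, controller, HUD, camera manager and game instance.
; The character is found by the Character.Player gameplay tag, while the controller (player index 0) and game instance are cast to PNC classes, printing a message on failure.
; HUD, camera manager and input toggling go through the controller, and IsPlayerCharacter compares a given character with the tagged one.
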(fn GetPNCCharacter
  (bind (_returncharacter _return) (CallFunction|GetCharacterbyTag "(TagName=\"Character.Player\")"))
  ;[0.5015 0.7837 1 0.3] Return a reference to the players character with the 'Character.Player' tag
  (if _return
    (return _returncharacter)
    (else
      (CallFunction|CustomPrint "Failed to find actor within the scene with 'Character.Player' tag" "NewEnumerator4" false)
      (return 0))))

(fn GetPNCPlayerController
  ;[0.5015 0.7837 1 0.3] Return a reference to the PNC Player Controller
  (bind _asbp_pncplayer_controller (Utilities|Casting|CastToBP_PNCPlayerController (Game|GetPlayerController 0))
    (:then
      (return _asbp_pncplayer_controller))
    (:CastFailed
      (CallFunction|CustomPrint "Failed to cast to PNCPlayerController" "NewEnumerator4" false)
      (return 0))))

(fn IsPlayerCharacter
  (params (Character :type Character%20Object%20Reference))
  ;[0.5015 0.7837 1 0.3] Checks to see if the in character is the same as the players character
  (return (== Character (CallFunction|GetPNCCharacter))))

(fn SetPlayerInput
  (params (Enabled :type Boolean))
  (bind _controller (CallFunction|GetPNCPlayerController))
  ;[0.5015 0.7837 1 0.3] Quick and easy to use function to Enable/Disable player input
  (Utilities|IsValid _controller
    (:Is%20Valid
      (Default|SetInputEnabled _controller Enabled))
    (:Is%20Not%20Valid
      _))
  (return))

(fn GetPlayerUI
  (bind _controller (CallFunction|GetPNCPlayerController))
  (bind _playerhud (Variables|/Game/PNCTookit/Blueprints/BP_PNCPlayerController.BP_PNCPlayerController_C|GetPlayerHUD _controller))
  ;[0.5015 0.7837 1 0.3] Quick and Easy function to return a reference to the 'Player Game UI'
  (Utilities|IsValid _playerhud
    (:Is%20Valid
      (return _playerhud))
    (:Is%20Not%20Valid
      (return 0))))

(fn GetPNCCameraManager
  ;[0.5015 0.7837 1 0.3] Return a reference to the players current camera manager
  (return (Variables|/Game/PNCTookit/Blueprints/BP_PNCPlayerController.BP_PNCPlayerController_C|GetCameraManagerRef (CallFunction|GetPNCPlayerController))))

(fn GetPNCGameInstance
  ;[0.5015 0.7837 1 0.3] Return a reference to the PNC Player Controller
  (bind _asbp_pncgame_instance (Utilities|Casting|CastToBP_PNCGameInstance (Game|GetGameInstance))
    (:then
      (return _asbp_pncgame_instance))
    (:CastFailed
      (CallFunction|CustomPrint "Failed to cast to game instance" "NewEnumerator5" false)
      (return 0))))