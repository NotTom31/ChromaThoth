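; BP_Tree is a non-pickup interactable tree in the point-and-click forest demo that the player can cut down with an axe.
; Using it starts the "CutDownTree" dialogue sequence.
; Receiving the Axe item consumes it and plays a timeline that rotates the tree mesh around its roll axis to animate the fall, while other items are rejected.
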(event Custom|TreeFallAnim
  (bind _rotx (Timeline|TreeFall Play)
    (:Update
      (Transformation|SetRelativeRotation (Variables|Default|GetTreemesh) (Math|Rotator|MakeRotator _rotx 0.0 0.0) false false))))

(fn ConstructionScript
  (|CallParentFunction))

(fn UseObject
  (params (InteractingCharacter :type BP%20PNC%20Character%20Parent%20Object%20Reference))
  (CallFunction|StartDialogueSequence "CutDownTree" InteractingCharacter)
  (return false))

(fn GetItemName
  (return "None"))

(fn IsInventoryItem
  (return false))

(fn Pickup
  (params (Instigator :type Actor%20Object%20Reference))
  (return false))

(fn RecieveItem
  (params (ItemName :type Name :default "None"))
  (switch name ItemName
    (:Default
      (return false false))
    (:Axe
      (CallFunction|TreeFallAnim)
      (return true true))))