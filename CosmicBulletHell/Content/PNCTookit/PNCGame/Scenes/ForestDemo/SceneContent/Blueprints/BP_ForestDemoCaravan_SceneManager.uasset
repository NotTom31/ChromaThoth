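; Scene manager for the forest demo's caravan scene, handling the shopkeeper's hidden state and introduction cutscene.
; Loading scene state strings teleports the shopkeeper to a hidden target point when flagged.
; The event-chained intro walks him to the counter, faces him and the player together, then plays dialogue on a counter camera.
; On completion it restores the camera, triggers his talk interaction and removes the hidden state.
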(event EventBeginPlay
  (|CallParentFunction) ; This node is disabled and will not be called.\nDrag off pins to build functionality.
)

(event Collision|EventActorBeginOverlap
  (params (OtherActor :type Actor%20Object%20Reference)))

(event EventTick
  (params (DeltaSeconds :type Float%20%28single-precision%29)))

(event Custom|ShopkeeperIntro
  ;[0.5728 1 0.9901 0.3] Introduce the shopkeeper to the player and move him to the
  (CallFunction|SetCutsceneState true)
  (Class|BPICharacter|MovetoLocation(Message) (Variables|Default|GetShopkeeperRef) (Transformation|GetActorLocation (Variables|Default|GetShopkeeperTargetPoint_Counter)))
  (EventDispatchers|BindEventtoOnMovementComplete (Variables|Default|GetShopkeeperRef) (delegate Custom|OnShopkeeperMoveComplete)))

(event Custom|SetShopkeeperHiddenLocation
  ;[0.5728 1 0.9901 0.3] Move the shopkeeper to the hidden storeroom location
  (Transformation|SetActorTransform (Variables|Default|GetShopkeeperRef) (Transformation|GetActorTransform (Variables|Default|GetShopkeeperTargetPoint_Hidden))))

(event Custom|OnShopkeeperMoveComplete
  (params (Character :type BP%20PNC%20Character%20Parent%20Object%20Reference))
  (bind _shopkeeperref (Variables|Default|GetShopkeeperRef))
  ;[0.5728 1 0.9901 0.3] Set the cutscene camera and Intro dialogue.
  (Class|BPICharacter|Lookat(Message) _shopkeeperref (Transformation|GetActorLocation (CallFunction|GetPNCCharacter)))
  (Class|BPICharacter|Lookat(Message) (CallFunction|GetPNCCharacter) (Transformation|GetActorLocation _shopkeeperref))
  (Game|Player|SetViewTargetwithBlend (CallFunction|GetPNCPlayerController) (Variables|Default|GetCounterCameraRef) 0.0 "VTBlend_Linear" 0.0 false)
  (bind _returnvalue (CallFunction|StartDialogueSequence "IntroShopkeeper"))
  (EventDispatchers|BindEventtoOnDialogueSequenceCompleteNotify _returnvalue (delegate Custom|OnDialogueComplete)))

(event Custom|OnDialogueComplete
  (bind _shopkeeperref (Variables|Default|GetShopkeeperRef))
  ;[0.5728 1 0.9901 0.3] End the cutscene
  (EventDispatchers|UnbindallEventsfromOnDialogueSequenceCompleteNotify (stale Custom|OnShopkeeperMoveComplete _returnvalue))
  (Game|Player|SetViewTargetwithBlend (CallFunction|GetPNCPlayerController) (CallFunction|GetPNCCameraManager) 0.0 "VTBlend_Linear" 0.0 false)
  (Class|BPIDialogue|Talkto(Message) _shopkeeperref _shopkeeperref "TalkToShopkeeper")
  (CallFunction|RemoveStateStringfromScene "" "ShopKeeperHidden"))

(fn ConstructionScript
  (|CallParentFunction))

(fn LoadStatefromStrings
  ;[1 0.6389 0.9805 0.3] Trigger available state from string.
  (for _array_element (Variables|Default|GetStateAsStrings)
    (switch string _array_element
      (:ShopKeeperHidden
        (CallFunction|SetShopkeeperHiddenLocation))))
  (return true))