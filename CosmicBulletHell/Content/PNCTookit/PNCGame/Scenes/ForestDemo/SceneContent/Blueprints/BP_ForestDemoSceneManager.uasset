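; Scene manager for the ForestDemo level, handling the main menu, intro cutscene and ending.
; The Forest Intro state string opens the menu or intro, depending on game state.
; The intro uses delays to sequence a camera blend, dialogue and credits, then brings the character through a door, clears the state and saves.
; The outro shows a "The End" title, then loads the main menu.
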(event Custom|BeginIntoCutscene
  ;[0.5813 1 0.5086 0.3] Begin Intro cutscene.
  (if (CallFunction|IsCutsceneEnabled)
    (Default|SetInputProfile (CallFunction|GetPNCPlayerController) "Gameplay")
    (Default|SetInputEnabled (CallFunction|GetPNCPlayerController) false) ; Disable player input
    (Transformation|SetActorTransform (CallFunction|GetPNCCharacter) (Transformation|GetActorTransform (Variables|IntroCutscene|GetIntroTargetPoint)))
    (Game|Player|SetViewTargetwithBlend (CallFunction|GetPNCPlayerController) (Variables|IntroCutscene|GetIntroCamera1) 0.0 "VTBlend_Linear" 0.0 false)
    (Game|Player|SetViewTargetwithBlend (CallFunction|GetPNCPlayerController) (CallFunction|GetPNCCameraManager) 45.0 "VTBlend_Cubic" 5.0 false)
    (Utilities|FlowControl|Delay 6.0)
    (CallFunction|StartDialogueSequence "IntroCharacter")
    (Utilities|FlowControl|Delay 11.0)
    (bind _returnvalue (UserInterface|CreateWidget "/Game/PNCTookit/PNCGame/Scenes/Shared/Widgets/WBP_OpeningCredits.WBP_OpeningCredits_C"))
    (bind _output_get (Variables|Default|SetOpeningCreditsWidgetRef _returnvalue))
    (UserInterface|Viewport|AddtoViewport _output_get 0)
    (Utilities|FlowControl|Delay 14.0)
    (CallFunction|StartDialogueSequence "IntroCallToAction")
    (Utilities|FlowControl|Delay 5.0)
    (CallFunction|IntroduceCharacter)))

(event Custom|IntroduceCharacter
  ;[0.5813 1 0.5086 0.3] Scripted player character introduction
  (Widget|RemovefromParent (Variables|Default|GetOpeningCreditsWidgetRef))
  (Default|ExitDoor (Variables|IntroCutscene|GetIntroDoorRef) (CallFunction|GetPNCCharacter))
  (CallFunction|RemoveStateStringfromScene "" "ForestIntro")
  (EventDispatchers|BindEventtoOnMovementComplete (CallFunction|GetPNCCharacter) (delegate Custom|OnMovementComplete)))

(event Custom|OnMovementComplete
  (params (Character :type BP%20PNC%20Character%20Parent%20Object%20Reference))
  ;[0.5813 1 0.5086 0.3] Scripted player character introduction
  (EventDispatchers|UnbindEventfromOnMovementComplete Character (delegate Custom|OnMovementComplete))
  (Default|SetInputEnabled (CallFunction|GetPNCPlayerController) false) ; Disable player input
  (CallFunction|UserSaveGame)
  (Utilities|FlowControl|Delay 4.0)
  (Default|SetInputEnabled (CallFunction|GetPNCPlayerController) true) ; Disable player input
)

(event Custom|BeginOutroCutscene
  ;[1 0.6592 0.3804 0.3] Play the outro cutscene.
  (if (CallFunction|IsCutsceneEnabled)
    (CallFunction|SetCutsceneState true)
    (bind _returnvalue (UserInterface|CreateWidget "/Game/PNCTookit/Blueprints/Widgets/Other/WBP_BasicSceneDisplayName.WBP_BasicSceneDisplayName_C"))
    (UserInterface|Viewport|AddtoViewport _returnvalue 0)
    (Default|InitSceneIntro _returnvalue 0 "The End")
    (Utilities|FlowControl|Delay 3.0)
    (Default|LoadMainMenu (CallFunction|GetPNCGameInstance))))

(event Custom|SetupMainMenu
  ;[1 1 1] Set the Main Menu state for the scene.
  (Default|SetInputProfile (CallFunction|GetPNCPlayerController) "Menu")
  (Game|Player|SetViewTargetwithBlend (CallFunction|GetPNCPlayerController) (Variables|IntroCutscene|GetIntroCamera1) 0.0 "VTBlend_Linear" 0.0 false)
  (bind _returnvalue (UserInterface|CreateWidget "/Game/PNCTookit/Blueprints/Widgets/Menus/WBP_MainMenu.WBP_MainMenu_C"))
  (bind _output_get (Variables|Default|SetMainMenuWidgetRef _returnvalue))
  (UserInterface|Viewport|AddtoViewport _output_get 0)
  (EventDispatchers|BindEventtoOnNewGame _output_get (delegate Custom|OnNewGame))
  (EventDispatchers|BindEventtoOnResumeGame (Variables|Default|GetMainMenuWidgetRef) (delegate Custom|OnResumeGame)))

(event Custom|OnNewGame
  ;[1 1 1] Set the Main Menu state for the scene.
  (EventDispatchers|UnbindallEventsfromOnNewGame (Variables|Default|GetMainMenuWidgetRef))
  (Widget|RemovefromParent (Variables|Default|GetMainMenuWidgetRef))
  (Variables|Default|SetMainMenuWidgetRef 0)
  (CallFunction|BeginIntoCutscene))

(event Custom|OnResumeGame
  ;[1 1 1] Set the Main Menu state for the scene.
  (EventDispatchers|UnbindallEventsfromOnResumeGame (Variables|Default|GetMainMenuWidgetRef))
  (Widget|RemovefromParent (Variables|Default|GetMainMenuWidgetRef))
  (Variables|Default|SetMainMenuWidgetRef 0))

(fn ConstructionScript
  (|CallParentFunction))

(fn LoadStatefromStrings
  ;[1 0.6389 0.9805 0.3] Trigger available state from string.
  (for _array_element (Variables|Default|GetStateAsStrings)
    (switch string _array_element
      (:ForestIntro
        (switch Utilities|FlowControl|Switch|SwitchonEGameState (Variables|/Game/PNCTookit/Blueprints/BP_PNCGameInstance.BP_PNCGameInstance_C|GetGameState (CallFunction|GetPNCGameInstance))
          (:NewEnumerator0
            (CallFunction|SetupMainMenu))
          (:NewEnumerator1
            (CallFunction|BeginIntoCutscene))))))
  (return false))