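; BP_Cooler is a usable, inspectable cooler in the ForestDemo scene that opens and closes its lid and can hold a referenced item.
; UseObject toggles IsUsed, playing or reversing one timeline that rotates the lid and fires events moving the item to show or hide it.
; First opening can start dialogue depending on the item, and inspection has its own line.
; LoadGameplayState reopens a used cooler and suppresses first-use dialogue.
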(event Custom|EventClose
  (bind _staticmesh (Variables|Default|GetStaticMesh))
  (bind _returnvalue (Transformation|GetWorldTransform _staticmesh))
  ;[0.3372 0.8148 1 0.298] Open/Close
  (bind _lidrotation (Timeline|LidAndTreeAnim Reverse)
    (:Update
      (Transformation|SetRelativeRotation (Variables|Default|GetLidMesh) (Math|Rotator|Lerp(Rotator) "0, 0, 0" "0, 0,-110.000000" _lidrotation) false false))
    (:HideItem
      ;[0.4062 0.7861 1 0.3] Hide item
      (bind _itemref (Variables|Gameplay|GetItemRef)
        (:then
          (Transformation|SetActorLocationAndRotation _itemref "0, 0, 0"))
        (:else)))
    (:ShowItem
      ;[0.4062 0.7861 1 0.3] Show Item
      (bind _itemref_2 (Variables|Gameplay|GetItemRef)
        (:then
          (Transformation|SetActorLocationAndRotation _itemref_2 (.location _returnvalue) (.rotation _returnvalue)))
        (:else)))))

(event Custom|EventOpen
  (bind _staticmesh (Variables|Default|GetStaticMesh))
  (bind _returnvalue (Transformation|GetWorldTransform _staticmesh))
  ;[0.3372 0.8148 1 0.298] Open/Close
  (bind _lidrotation (Timeline|LidAndTreeAnim Play)
    (:Update
      (Transformation|SetRelativeRotation (Variables|Default|GetLidMesh) (Math|Rotator|Lerp(Rotator) "0, 0, 0" "0, 0,-110.000000" _lidrotation) false false))
    (:HideItem
      ;[0.4062 0.7861 1 0.3] Hide item
      (bind _itemref (Variables|Gameplay|GetItemRef)
        (:then
          (Transformation|SetActorLocationAndRotation _itemref "0, 0, 0"))
        (:else)))
    (:ShowItem
      ;[0.4062 0.7861 1 0.3] Show Item
      (bind _itemref_2 (Variables|Gameplay|GetItemRef)
        (:then
          (Transformation|SetActorLocationAndRotation _itemref_2 (.location _returnvalue) (.rotation _returnvalue)))
        (:else)))))

(fn ConstructionScript
  (|CallParentFunction))

(fn UseObject
  (params (InteractingCharacter :type BP%20PNC%20Character%20Parent%20Object%20Reference))
  ;[0.5688 1 0.5048 0.3] When used Open/Close the lid of the cooler
  (if (Variables|Default|GetbIsUsed)
    (Variables|Default|SetbIsUsed false)
    (CallFunction|EventClose)
    (else
      (Variables|Default|SetbIsUsed true)
      (bind _itemref (Variables|Gameplay|GetItemRef)
        (:then
          (if (Variables|/Game/PNCTookit/Blueprints/Gameplay/Items/BP_ItemBase.BP_ItemBase_C|GetbIsActive _itemref)
            (if (Variables|Gameplay|GetbFirstInteraction)
              (CallFunction|StartDialogueSequence "UseCooler")
              (Variables|Gameplay|SetbFirstInteraction false))))
        (:else
          (if (Variables|Gameplay|GetbFirstInteraction)
            (CallFunction|StartDialogueSequence "UseCoolerEmpty")
            (Variables|Gameplay|SetbFirstInteraction false))))
      (CallFunction|EventOpen)))
  (return true))

(fn LoadGameplayState
  ;[1 0.9129 0.4825 0.3] If the cooler has already been used by the player, disable any dialogue and open the lid
  (if (Variables|Default|GetbIsUsed)
    (Variables|Gameplay|SetbFirstInteraction false)
    (CallFunction|EventOpen))
  (return true))

(fn OnInspection
  (params (Inspector :type Controller%20Object%20Reference))
  (CallFunction|StartDialogueSequence "InspectCooler")
  (return true))