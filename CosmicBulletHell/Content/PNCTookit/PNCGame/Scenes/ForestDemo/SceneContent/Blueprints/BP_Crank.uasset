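; BP_Crank is an interactable crank in the PNC toolkit's forest demo that operates a referenced stairs object.
; Each use toggles IsUsed, playing or reversing the StairsAnim timeline that pitches the handle mesh, then forwards the use to StairsRef and returns its result.
; Inspection starts the InspectCrank dialogue sequence, while pickup and item-receiving are stubbed out.
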(event Custom|UseHandleClose
  (bind (_direction _yrotation) (Timeline|StairsAnim ReverseFromEnd)
    (:Update
      (Transformation|SetRelativeRotation (Variables|Default|GetSM_Crank_Handle) (Math|Rotator|MakeRotator 0.0 _yrotation 0.0) false false))
    (:Finished
      (switch Utilities|FlowControl|Switch|SwitchonETimelineDirection _direction))))

(event Custom|UseHandleOpen
  (bind (_direction _yrotation) (Timeline|StairsAnim Play)
    (:Update
      (Transformation|SetRelativeRotation (Variables|Default|GetSM_Crank_Handle) (Math|Rotator|MakeRotator 0.0 _yrotation 0.0) false false))
    (:Finished
      (switch Utilities|FlowControl|Switch|SwitchonETimelineDirection _direction))))

(event EventBeginPlay
  (|CallParentFunction) ; This node is disabled and will not be called.\nDrag off pins to build functionality.
)

(event Collision|EventActorBeginOverlap
  (params (OtherActor :type Actor%20Object%20Reference)))

(event EventTick
  (params (DeltaSeconds :type Float%20%28single-precision%29)))

(fn ConstructionScript
  (|CallParentFunction))

(fn UseObject
  (params (InteractingCharacter :type BP%20PNC%20Character%20Parent%20Object%20Reference))
  (if (Variables|Default|GetbIsUsed)
    (Variables|Default|SetbIsUsed false)
    (CallFunction|UseHandleClose)
    (else
      (Variables|Default|SetbIsUsed true)
      (CallFunction|UseHandleOpen)))
  (bind _success (Class|BPIObjectInteractions|UseObject(Message) (Variables|Default|GetStairsRef) InteractingCharacter))
  (return _success))

(fn OnInspection
  (params (Inspector :type Controller%20Object%20Reference))
  (CallFunction|StartDialogueSequence "InspectCrank" Inspector)
  (return false))

(fn GetItemName
  (return "None"))

(fn IsInventoryItem
  (return false))

(fn Pickup
  (params (Instigator :type Actor%20Object%20Reference))
  (return false))

(fn RecieveItem
  (params (ItemName :type Name :default "None"))
  (return false false))