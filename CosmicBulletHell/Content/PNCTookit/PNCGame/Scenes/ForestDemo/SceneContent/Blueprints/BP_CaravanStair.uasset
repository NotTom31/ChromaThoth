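; BP_CaravanStair is a usable caravan stair in the ForestDemo scene that toggles between raised and dropped.
; UseObject flips IsUsed through SetStairState, and LoadGameplayState reapplies that value on load.
; Dropping plays the StairsAnim timeline to rotate the mesh, while raising reverses it from the end.
; A NavModifier switches between default and null area classes, so navigation is open only while the stair is down.
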(event Custom|RaiseStairs
  (Class|NavModifierComponent|SetAreaClass (Variables|Default|GetNavModifier) "/Script/NavigationSystem.NavArea_Null")
  (bind _alpha (Timeline|StairsAnim ReverseFromEnd)
    (:Update
      (Transformation|SetRelativeRotation (Variables|Default|GetMesh) (Math|Rotator|Lerp(Rotator) "0, 0,-104.062332" "0, 0, 0" _alpha true) false false))))

(event Custom|DropStairs
  (Class|NavModifierComponent|SetAreaClass (Variables|Default|GetNavModifier) "/Script/NavigationSystem.NavArea_Default")
  (bind _alpha (Timeline|StairsAnim Play)
    (:Update
      (Transformation|SetRelativeRotation (Variables|Default|GetMesh) (Math|Rotator|Lerp(Rotator) "0, 0,-104.062332" "0, 0, 0" _alpha true) false false))))

(event EventBeginPlay
  (|CallParentFunction))

(event Collision|EventActorBeginOverlap
  (params (OtherActor :type Actor%20Object%20Reference)))

(event EventTick
  (params (DeltaSeconds :type Float%20%28single-precision%29)))

(fn ConstructionScript
  (|CallParentFunction))

(fn UseObject
  (params (InteractingCharacter :type BP%20PNC%20Character%20Parent%20Object%20Reference))
  (if (Variables|Default|GetbIsUsed)
    (CallFunction|SetStairState false)
    (else
      (CallFunction|SetStairState true)))
  (return true))

(fn SetStairState
  (params (bIsUsed :type Boolean))
  (bind _output_get (Variables|Default|SetbIsUsed bIsUsed))
  (if _output_get
    (CallFunction|DropStairs)
    (else
      (CallFunction|RaiseStairs))))

(fn LoadGameplayState
  (CallFunction|SetStairState (Variables|Default|GetbIsUsed))
  (return true))