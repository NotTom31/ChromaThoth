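; BP_Door_CaravanExterior is the caravan's exterior door in the ForestDemo scene, usable only after the referenced stairs have been used.
; Its UseObject override checks StairsRef.IsUsed and, when true, defers to the parent's use logic and returns that result.
; Otherwise it starts the "UseStoreDoorUnreachable" dialogue sequence and returns false.
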(event EventBeginPlay
  (|CallParentFunction) ; This node is disabled and will not be called.\nDrag off pins to build functionality.
)

(event Collision|EventActorBeginOverlap
  (params (OtherActor :type Actor%20Object%20Reference)))

(event EventTick
  (params (DeltaSeconds :type Float%20%28single-precision%29)))

(fn ConstructionScript
  (|CallParentFunction))

(fn UseObject
  (params (InteractingCharacter :type BP%20PNC%20Character%20Parent%20Object%20Reference))
  (if (Variables|/Game/PNCTookit/Blueprints/Gameplay/Scene/BP_InteractableObjectBase.BP_InteractableObjectBase_C|GetbIsUsed (Variables|Default|GetStairsRef))
    (bind _success (|CallParentFunction InteractingCharacter))
    (return _success)
    (else
      (CallFunction|StartDialogueSequence "UseStoreDoorUnreachable")
      (return false))))