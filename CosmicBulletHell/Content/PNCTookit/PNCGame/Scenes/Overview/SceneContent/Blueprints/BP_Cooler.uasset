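; Interactable cooler Blueprint that toggles open and closed on use, with an item snapped to its scene component.
; A single timeline swings the lid and scales a tree mesh, playing to open and reversing to close.
; UseObject flips IsUsed and the item's active state, while LoadGameplayState reopens a used cooler without updating the item.
; The open and close sound nodes are disconnected, so the PlaySound flag has no effect.
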(event Custom|EventClose
  ;[0.3372 0.8148 1 0.298] Open/Close
  (bind (_direction _lidrotation _treescale) (Timeline|LidAndTreeAnim Reverse)
    (:Update
      (Transformation|SetRelativeRotation (Variables|Default|GetLidMesh) (Math|Rotator|Lerp(Rotator) "0, 0, 0" "0, 0,-110.000000" _lidrotation) false false)
      (Transformation|SetRelativeScale3D (Variables|Default|GetTreeMesh) (Math|Conversions|ToVector(Float) (* (Variables|Gameplay|GetTreeScale) _treescale))))
    (:Finished
      (switch Utilities|FlowControl|Switch|SwitchonETimelineDirection _direction))))

(event Custom|EventOpen
  (params (PlaySound :type Boolean))
  ;[0.3372 0.8148 1 0.298] Open/Close
  (if PlaySound
    (bind (_direction _lidrotation _treescale) (Timeline|LidAndTreeAnim Play)
      (:Update
        (Transformation|SetRelativeRotation (Variables|Default|GetLidMesh) (Math|Rotator|Lerp(Rotator) "0, 0, 0" "0, 0,-110.000000" _lidrotation) false false)
        (Transformation|SetRelativeScale3D (Variables|Default|GetTreeMesh) (Math|Conversions|ToVector(Float) (* (Variables|Gameplay|GetTreeScale) _treescale))))
      (:Finished
        (switch Utilities|FlowControl|Switch|SwitchonETimelineDirection _direction)))
    (else
      (Timeline|LidAndTreeAnim Play))))

(event EventBeginPlay
  ;[1 0.9046 0.3931 0.3] Attach Item to scene component
  (|CallParentFunction)
  (Transformation|AttachComponentToComponent (Variables|Default|GetItemRef) (Variables|Default|GetScene) "None" "SnapToTarget" "SnapToTarget" "SnapToTarget" false))

(fn ConstructionScript
  (|CallParentFunction))

(fn UseObject
  (params (InteractingCharacter :type BP%20PNC%20Character%20Parent%20Object%20Reference))
  ;[0.5688 1 0.5048 0.3] When used Open/Close the lid of the cooler
  (if (Variables|Default|GetbIsUsed)
    (Variables|Default|SetbIsUsed false)
    (CallFunction|EventClose)
    (Default|SetItemActiveState (Variables|Default|GetItemRef) false)
    (else
      (Variables|Default|SetbIsUsed true)
      (CallFunction|EventOpen true)
      (Default|SetItemActiveState (Variables|Default|GetItemRef) true)))
  (return true))

(fn LoadGameplayState
  ;[1 0.9129 0.4825 0.3] If the cooler has already been used by the player, disable any dialogue and open the lid
  (if (Variables|Default|GetbIsUsed)
    (CallFunction|EventOpen false))
  (return true))