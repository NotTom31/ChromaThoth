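; BP_BasicInteractableObject is an interactable object for the point-and-click toolkit's Overview scene that shakes and talks when used.
; UseObject ignores use while the shake timeline plays, otherwise defers to the parent implementation.
; On parent success it triggers PlayShakeAnim and starts a dialogue sequence from a randomly chosen RandomDialogue row.
; The timeline drives the mesh's relative location and rotation.
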(event Custom|PlayShakeAnim
  ;[0.4574 1 0.9701 0.3] Play Shake Anim
  (bind (_direction _location _rotation) (Timeline|ShakeAnim PlayFromStart)
    (:Update
      (Transformation|SetRelativeTransform (Variables|Default|GetMesh) (Math|Transform|MakeTransform _location (Math|Rotator|MakeRotator (.x _rotation) (.y _rotation) (.z _rotation))) false false))))

(fn ConstructionScript
  (|CallParentFunction))

(fn UseObject
  (params (InteractingCharacter :type BP%20PNC%20Character%20Parent%20Object%20Reference))
  (if (not (Audio|Components|Audio|IsPlaying (Variables|Default|GetShakeAnim)))
    (bind _success (|CallParentFunction InteractingCharacter))
    (if _success
      (CallFunction|PlayShakeAnim)
      (CallFunction|StartDialogueSequence (Utilities|Array|Get(acopy) (Variables|Default|GetRandomDialogue) (Math|Random|RandomIntegerinRange 0 2)) self))
    (return _success)
    (else
      (return false))))