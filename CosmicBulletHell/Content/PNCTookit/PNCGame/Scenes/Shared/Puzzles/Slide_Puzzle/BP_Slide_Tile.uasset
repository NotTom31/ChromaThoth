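; BP_Slide_Tile is a single clickable piece of a sliding tile puzzle, initialized with an ID and a parent puzzle.
; InitTile uses the ID to pick the mesh material and set the text label, and clicks forward the tile to the parent's SlideTile.
; IsColliding tests a given component for overlaps with other tiles or the puzzle.
; Actor collision starts disabled, and DropTile briefly simulates physics before destroying the tile.
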(event Custom|DropTile
  (Collision|SetActorEnableCollision false)
  (Physics|SetSimulatePhysics (Variables|Default|GetSM_Sign_Map_Puzzle_Piece) true)
  (Utilities|FlowControl|Delay 0.5)
  (Actor|DestroyActor))

(event MouseInput|EventActorOnClicked
  (params (ButtonPressed :type Key%20Structure))
  (bind _parent (Variables|Default|GetParent))
  (Utilities|IsValid _parent
    (:Is%20Valid
      (Default|SlideTile _parent self))))

(event EventBeginPlay
  (Collision|SetActorEnableCollision false))

(fn ConstructionScript)

(fn IsColliding
  (params (CollisionComponent :type Primitive%20Component%20Object%20Reference))
  (return (or (>= (Utilities|Array|Length (Collision|GetOverlappingActors CollisionComponent "BP_Slide_Tile_C" :!class /Script/Engine.PrimitiveComponent)) 1) (>= (Utilities|Array|Length (Collision|GetOverlappingActors CollisionComponent "/Game/PNCTookit/PNCGame/Scenes/Shared/Puzzles/Slide_Puzzle/BP_Slide_Puzzle.BP_Slide_Puzzle_C" :!class /Script/Engine.PrimitiveComponent)) 1))))

(fn InitTile
  (params (Parent :type BP%20Slide%20Puzzle%20Object%20Reference) (ID :type Integer))
  (Variables|Default|SetParent Parent)
  (Variables|Default|SetTileID ID)
  (Rendering|Material|SetMaterial (Variables|Default|GetSM_Sign_Map_Puzzle_Piece) 0 (Utilities|Array|Get(acopy) (Variables|Default|GetTextureArray) (Variables|Default|GetTileID)))
  (Rendering|Components|TextRender|SetText (Variables|Default|GetTextRender) (Utilities|Text|FormatText "{id}" (Variables|Default|GetTileID))))