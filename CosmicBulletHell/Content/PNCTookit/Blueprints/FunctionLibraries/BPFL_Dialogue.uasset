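; Blueprint function library of dialogue helpers for the PNC toolkit, starting sequences and resolving their data.
; StartDialogueSequence passes a row name and initiator to the Dialogue Manager widget held by the PNC player controller.
; GetDialogueSequence searches the scene manager's active dialogue data tables, plus defaults, for the row, printing debug hints on failure.
; GetActorDialoguePosition projects an actor's dialogue-position component to screen coordinates, returning false when absent.
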(fn StartDialogueSequence
  (params (DialogueRowName :type Name) (InitiatingActor :type Actor%20Object%20Reference))
  (bind _dialogmanager (CallFunction|GetPlayerDialogueManagerRef))
  (Default|BeginDialogueSequence _dialogmanager DialogueRowName InitiatingActor)
  (return _dialogmanager))

(fn GetPlayerDialogueManagerRef
  (bind _controller (CallFunction|GetPNCPlayerController))
  (bind _dialoguemanager (Variables|/Game/PNCTookit/Blueprints/BP_PNCPlayerController.BP_PNCPlayerController_C|GetDialogueManager _controller))
  ;[0.5374 0.9401 1 0.3] Returns a reference to the players Dialogue Manager Widget
  (Utilities|IsValid _controller
    (:Is%20Valid
      (Utilities|IsValid _dialoguemanager
        (:Is%20Valid
          (return _dialoguemanager))))
    (:Is%20Not%20Valid
      (return 0))))

(fn GetDialogueSequence
  (params (RowName :type Name))
  ;[1 0.8886 0.3571 0.3] Return a valid dialogue sequece struct from the given sequence name. Only Active Dialogue Data tables (in the scene manager) will be checked.
  (Utilities|Array|AppendArray (LocalVariables|GetActiveDialogueDataTables) (Variables|/Game/PNCTookit/Blueprints/BP_SceneManagerBase.BP_SceneManagerBase_C|GetActiveDialogueDataTables (CallFunction|GetSceneManager)))
  (for _array_element (LocalVariables|GetActiveDialogueDataTables)
    (bind _outrownames (DataTable|GetDataTableRowNames _array_element))
    (if (Utilities|Array|ContainsItem _outrownames RowName)
      (bind _returnvalue (Utilities|GetDataTableRow _array_element RowName)
        (:then
          (return true _returnvalue))
        (:RowNotFound
          (return false "")))))
  (CallFunction|CustomPrint "Dialogue Row Name could not be found." "NewEnumerator4" true)
  (CallFunction|CustomPrint "Tip: Maybe your dialogue data table has not been added 
to your active list(?) in the Game Mode." "NewEnumerator3" true)
  (return false ""))

(fn GetActorDialoguePosition
  (params (Actor :type Actor%20Object%20Reference))
  (bind _returnvalue (Actor|GetComponentbyClass Actor "/Game/PNCTookit/Blueprints/Components/BP_DialoguePositionSceneComponent.BP_DialoguePositionSceneComponent_C"))
  (bind _controller (CallFunction|GetPNCPlayerController))
  (bind _returnvalue_2 (Transformation|GetWorldLocation _returnvalue))
  (bind _screenposition (Class|GameplayStatics|ProjectWorldtoScreen _controller _returnvalue_2 false))
  ;[1 0.9321 0.3896 0.3] Get an actors dialogue position on screen
  (Utilities|IsValid Actor
    (:Is%20Valid
      (Utilities|IsValid _returnvalue
        (:Is%20Valid
          (return (Math|Vector2D|MakeVector2D (.x _screenposition) (.y _screenposition)) true))
        (:Is%20Not%20Valid
          (return "" false))))
    (:Is%20Not%20Valid
      (return "" false))))

(fn GetDialogueManagerRef
  ;[0.5015 0.7837 1 0.3] Return a reference to the players Dialogue Manager
  (return (Variables|/Game/PNCTookit/Blueprints/BP_PNCPlayerController.BP_PNCPlayerController_C|GetDialogueManager (CallFunction|GetPNCPlayerController))))