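; Blueprint function library of small vector math helpers in the PNC toolkit.
; It clamps 3D and 2D vectors per component and finds the midpoint between two vectors.
; IsVector2DInRange tests whether a 2D value is near a goal on each axis within a fixed tolerance, and also outputs the difference between their lengths.
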(fn ClampVector
  (params (Value :type Vector) (Min :type Vector) (Max :type Vector))
  (bind (_x _y _z) (Math|Vector|BreakVector Max))
  (bind (_x_2 _y_2 _z_2) (Math|Vector|BreakVector Value))
  (bind (_x_3 _y_3 _z_3) (Math|Vector|BreakVector Min))
  (return (Math|Vector|MakeVector (Math|Float|Clamp(Float) _x_2 _x_3 _x) (Math|Float|Clamp(Float) _y_2 _y_3 _y) (Math|Float|Clamp(Float) _z_2 _z_3 _z))))

(fn GetCenterPointOfVectors
  (params (A :type Vector) (B :type Vector))
  (return (/ (+ A B) 2.0)))

(fn IsVector2DinRange
  (params (Value :type Vector%202D%20Structure) (Goal :type Vector%202D%20Structure))
  (bind _returnvalue (Math|Float|MakeLiteralFloat 1e+02))
  (bind (_x _y) (Math|Vector2D|BreakVector2D Goal))
  (bind (_x_2 _y_2) (Math|Vector2D|BreakVector2D Value))
  (return (and (Math|Float|NearlyEqual(Float) _x_2 _x _returnvalue) (Math|Float|NearlyEqual(Float) _y_2 _y _returnvalue)) (- (Math|Vector2D|Vector2DLength Value) (Math|Vector2D|Vector2DLength Goal))))

(fn ClampVector2D
  (params (Value :type Vector%202D%20Structure) (Min :type Vector%202D%20Structure) (Max :type Vector%202D%20Structure))
  (bind (_x _y) (Math|Vector2D|BreakVector2D Max))
  (bind (_x_2 _y_2) (Math|Vector2D|BreakVector2D Value))
  (bind (_x_3 _y_3) (Math|Vector2D|BreakVector2D Min))
  (return (Math|Vector2D|MakeVector2D (Math|Float|Clamp(Float) _x_2 _x_3 _x) (Math|Float|Clamp(Float) _y_2 _y_3 _y))))