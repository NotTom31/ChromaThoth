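; BPFL_DeveloperHelpers is a Blueprint function library providing a Custom Print helper for categorized developer messages.
; It prefixes each string with its uppercased log type in brackets and picks a text color per type, keeping Log-type messages off screen.
; Messages flagged as Debug print only when debug messages are enabled, while others always print.
; An unconnected StackTrace branch into the print never runs.
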(fn CustomPrint
  (params (String :type String) (LogType :type ELogVerbosityEnum%20Enum :default "NewEnumerator0") (Debug :type Boolean))
  (if (LocalVariables|GetIsDebugMessageEnabled)
    (Development|PrintString 0 (Utilities|String|Append "" (Utilities|String|Append "[" (Class|KismetStringLibrary|ToUpper (Utilities|String|EnumtoString LogType)) "]   ") String) (Utilities|Select :Index LogType :NewEnumerator0 false :NewEnumerator3 true :NewEnumerator4 true :NewEnumerator5 true :NewEnumerator6 true) true (Utilities|Select :Index LogType :NewEnumerator0 "(R=0.000000,G=0.665387,B=1.000000,A=1.000000)" :NewEnumerator3 "(R=0.000000,G=1.000000,B=0.000000,A=1.000000)" :NewEnumerator4 "(R=1.000000,G=0.349979,B=0.000000,A=1.000000)" :NewEnumerator5 "(R=1.000000,G=0.000000,B=0.000000,A=1.000000)" :NewEnumerator6 "(R=1.000000,G=0.000000,B=0.000000,A=1.000000)") 1e+01 :!label _label)
    (elif (not Debug)
      (goto _label))))