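; Blueprint function library of navigation helpers for the PNC toolkit's movement and actor interaction.
; Resolves an interactable's interaction volume through the interaction manager to a raised navmesh point, falling back to the actor's location.
; Also validates paths, checks range by volume overlap or distance, and sphere-traces from the mouse to project a navmesh point.
; A separate helper snaps yaw into four- or eight-way 2D look directions.
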(fn GetInteractionVolume
  (params (InteractableActor :type Actor%20Object%20Reference))
  (bind _return (CallFunction|GetInteractionManager))
  ;[1 0.923 0.4664 0.3] Return the location (on navmesh) of a valid interaction volume. If Invalid this will just return the location of the actor itself (Default still returns invalid)
  (Utilities|IsValid InteractableActor
    (:Is%20Valid
      (LocalVariables|SetInteractingActorRef InteractableActor)
      (Utilities|IsValid _return
        (:Is%20Valid
          (Utilities|IsValid (Default|GetActorsInteractionVolume _return (LocalVariables|GetInteractingActorRef))
            (:Is%20Valid
              (return (Default|GetActorsInteractionVolume _return (LocalVariables|GetInteractingActorRef)) (.NavLocation (CallFunction|GetClosestNavPointatLocation (Transformation|GetActorLocation (Default|GetActorsInteractionVolume _return (LocalVariables|GetInteractingActorRef))))) (.Return (CallFunction|GetClosestNavPointatLocation (Transformation|GetActorLocation (Default|GetActorsInteractionVolume _return (LocalVariables|GetInteractingActorRef)))))))
            (:Is%20Not%20Valid
              _)))
        (:Is%20Not%20Valid
          _))
      (return 0 (.NavLocation (CallFunction|GetClosestNavPointatLocation (Transformation|GetActorLocation (LocalVariables|GetInteractingActorRef)))) (.Return (CallFunction|GetClosestNavPointatLocation (Transformation|GetActorLocation (LocalVariables|GetInteractingActorRef))))))
    (:Is%20Not%20Valid
      (return 0 "0, 0, 0" true))))

(fn TestNavigationPath
  (params (PathStartLocation :type Vector) (PathEndLocation :type Vector) (PathFindingContext :type Actor%20Object%20Reference))
  ;[1 0.923 0.4664 0.3] Test the navigtion path to see if there are any valid path points returned
  (LocalVariables|SetEndLocation PathStartLocation)
  (bind _returnvalue (Class|NavigationSystemV1|FindPathtoLocationSynchronously 0 PathStartLocation PathEndLocation PathFindingContext 0))
  (Utilities|IsValid _returnvalue
    (:Is%20Valid
      (if (>= (Utilities|Array|Length (Variables|/Script/NavigationSystem.NavigationPath|GetPathPoints _returnvalue)) 1)
        _
        (else
          (CallFunction|CustomPrint "Invalid navigation path (No path Points Found)" "NewEnumerator0" false)))
      (return (>= (Utilities|Array|Length (Variables|/Script/NavigationSystem.NavigationPath|GetPathPoints _returnvalue)) 1)))
    (:Is%20Not%20Valid
      (return false))))

(fn InteractionVolumeWithinRange
  (params (Actor%20A :type Actor%20Object%20Reference) (Actor%20B :type Actor%20Object%20Reference))
  ;[1 0.923 0.4664 0.3] Check to see if there is a valid interaction volume within range of actor A
  (for _array_element (Collision|GetOverlappingActors Actor%20A "/Game/PNCTookit/Blueprints/Gameplay/Scene/BP_InteractionVolume.BP_InteractionVolume_C" :!class /Script/Engine.Actor)
    (if (== _array_element (.InteractionVolumes (CallFunction|GetInteractionVolume Actor%20B)))
      (return true)))
  (return false))

(fn SphereTracetoNavMesh
  (params (PlayerController :type Player%20Controller%20Object%20Reference) (FailedMoveLocationTraceExtent :type Float%20%28single-precision%29))
  ;[1 0.923 0.4664 0.3] Sphere trace into the scene for a valid navmesh point
  (bind (_outhit _returnvalue) (Collision|SphereTraceForObjects 0 (CallFunction|MousetoWorldPosition PlayerController 0.0) (CallFunction|MousetoWorldPosition PlayerController 7e+03) FailedMoveLocationTraceExtent (Utilities|Array|MakeArray "ObjectTypeQuery2") false 0 "None" true "(R=1.000000,G=0.000000,B=0.000000,A=1.000000)" "(R=0.000000,G=1.000000,B=0.000000,A=1.000000)" 2.0))
  (return (.ProjectedLocation (AI|Navigation|ProjectPointtoNavigation 0 (* (.ImpactPoint (Collision|BreakHitResult _outhit)) "1.000000,1.000000,0.000000") 0 0 (Math|Conversions|ToVector(Float) FailedMoveLocationTraceExtent))) _returnvalue))

(fn Get2DLookatDirection
  (params (Rotation :type Rotator) (IncludeDiagonalDirections :type Boolean))
  (bind _yaw (Math|Rotator|BreakRotator Rotation))
  (bind _returnvalue (/ 3.6e+02 8.0))
  (bind _returnvalue_2 (select IncludeDiagonalDirections 1.0 2.0))
  (bind _returnvalue_3 (* _returnvalue _returnvalue_2))
  (bind _returnvalue_4 (Math|Float|SnapToGrid(Float) _yaw _returnvalue_3))
  (bind _returnvalue_5 (+ _returnvalue_4 1.8e+02))
  (bind _returnvalue_6 (Math|Float|Absolute(Float) _returnvalue_5))
  (bind _returnvalue_7 (/ _returnvalue_6 _returnvalue_3))
  (bind _returnvalue_8 (Math|Float|Floor _returnvalue_7))
  ;[1 0.923 0.4664 0.3] Return a 2D look at Direction based on the rotation input
  (Utilities|FlowControl|Sequence
    (:then_0
      (if IncludeDiagonalDirections
        (switch int _returnvalue_8
          (:0
            (LocalVariables|SetReturnDirection "NewEnumerator6" :!label _label))
          (:1
            (LocalVariables|SetReturnDirection "NewEnumerator1"))
          (:2
            (LocalVariables|SetReturnDirection "NewEnumerator0" :!label _label_2))
          (:3
            (LocalVariables|SetReturnDirection "NewEnumerator2"))
          (:4
            (LocalVariables|SetReturnDirection "NewEnumerator7" :!label _label_3))
          (:5
            (LocalVariables|SetReturnDirection "NewEnumerator5"))
          (:6
            (LocalVariables|SetReturnDirection "NewEnumerator3" :!label _label_4))
          (:7
            (LocalVariables|SetReturnDirection "NewEnumerator4"))
          (:8
            (goto _label)))
        (else
          (switch int _returnvalue_8
            (:0
              (goto _label))
            (:1
              (goto _label_2))
            (:2
              (goto _label_3))
            (:3
              (goto _label_4))))))
    (:then_1
      (return (LocalVariables|GetReturnDirection) (Math|Rotator|MakeRotator 0.0 0.0 _returnvalue_4)))))

(fn GetClosestNavPointatLocation
  (params (Location :type Vector))
  (bind _projectedlocation (AI|Navigation|ProjectPointtoNavigation 0 Location 0 0 "500.000000,500.000000,500.000000"))
  (bind _returnvalue (+ _projectedlocation "0, 0,50.000000"))
  ;[1 0.923 0.4664 0.3] Find the closest point on the navmesh for the input location
  (if (Math|Vector|NotEqual(Vector) _projectedlocation "0, 0, 0" 0.0001)
    (return _returnvalue true)
    (else
      (CallFunction|CustomPrint "\"Get Closest Nav Point At Location\" funtion failed to get a valid navigation point and returned X = 0.0 , Y = 0.0, Z = 0.0" "NewEnumerator0" true)
      (return _returnvalue false))))

(fn ActorWithinRange
  (params (FromActor :type Actor%20Object%20Reference) (TargetActor :type Actor%20Object%20Reference) (Distance :type Float%20%28single-precision%29))
  ;[1 0.923 0.4664 0.3] Similar to 'Interaction Volume in Range', this checks to see to see if the actors are within a distance range to the target actor.
  (if (and (Utilities|IsValid FromActor) (Utilities|IsValid TargetActor))
    (return (<= (Math|Vector|VectorLength (- (Transformation|GetActorLocation FromActor) (Transformation|GetActorLocation TargetActor))) Distance))
    (else
      (return false))))