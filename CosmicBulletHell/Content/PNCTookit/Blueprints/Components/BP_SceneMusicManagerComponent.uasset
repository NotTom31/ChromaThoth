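; Scene music manager component that plays 2D background music and transitions between tracks.
; PlayMusic ignores invalid or unchanged sounds, otherwise stores the track and volume, stops any current audio, waits the fade-out duration, then spawns and fades in the new sound.
; StopMusic calls FadeOut but destroys the audio component immediately afterwards, without waiting for the fade to finish.
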(event Custom|PlayMusic
  (params (Music :type Sound%20Wave%20Object%20Reference) (Volume :type Float%20%28single-precision%29))
  ;[0.4297 0.9101 1 0.3] Transition and play the given sound wave
  (if (and (Utilities|IsValid Music) (!= Music (Variables|Default|GetMusicRef)))
    (Variables|Default|SetMusicRef Music)
    (Variables|Default|SetVolume Volume)
    (Utilities|IsValid (Variables|Default|GetMusicAudioComponent)
      (:Is%20Valid
        (CallFunction|StopMusic)
        (Utilities|FlowControl|Delay (Variables|Default|GetFadeOutDuration)))
      (:Is%20Not%20Valid
        _))
    (bind _returnvalue (Audio|SpawnSound2D (Variables|Default|GetMusicRef) 1.0 1.0 0.0 0))
    (bind _output_get (Variables|Default|SetMusicAudioComponent _returnvalue))
    (Audio|Components|Audio|FadeIn _output_get (Variables|Default|GetFadeInDuration) (Variables|Default|GetVolume) 0.0 :!class /Script/Engine.AudioComponent)))

(fn StopMusic
  (Audio|Components|Audio|FadeOut (Variables|Default|GetMusicAudioComponent) (Variables|Default|GetFadeOutDuration) 0.0 :!class /Script/Engine.AudioComponent)
  (Components|DestroyComponent (Variables|Default|GetMusicAudioComponent)))