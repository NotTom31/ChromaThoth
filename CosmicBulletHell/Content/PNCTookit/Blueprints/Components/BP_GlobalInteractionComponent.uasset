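; BP_GlobalInteractionComponent is a component that gives its owning interactive actor instance a unique GUID for use in save games.
; GenerateGUID assigns a new GUID only when the current one is all zeros or the caller forces replacement.
; Each new assignment prints a warning with the owner's display name and calls a stack trace, exposing where identifiers change.
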(fn GenerateGUID
  (params (ReplaceValid :type Boolean))
  ;[0.4913 0.6396 1 0.3] Generate a new unique identifier for this interactive actor instance. Used for Save Games.
  (if (or (== (Variables|SaveGame|GetGUID) (.OutGuid (Class|KismetGuidLibrary|ParseStringtoGuid "{00000000-0000-0000-0000-000000000000}"))) ReplaceValid)
    (Variables|SaveGame|SetGUID (Guid|NewGuid))
    (Development|PrintString (Utilities|String|Append "WARNING: NEW GUID = " (Utilities|GetDisplayName (Components|GetOwner))))
    (Class|KismetSystemLibrary|StackTrace)))