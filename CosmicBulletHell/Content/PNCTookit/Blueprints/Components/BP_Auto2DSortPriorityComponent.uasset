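; Actor component that auto-sorts the 2D draw order of its owner's Paper2D flipbook and sprite components.
; Sets each component's translucent sort priority to a truncated world Y, taken from either the owning actor or the component itself.
; With dynamic sorting on, BeginPlay enables tick and runs the sort, which Tick then repeats every frame.
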(event EventBeginPlay
  (if (Variables|Default|GetbDynamicSortingOnTick)
    (Components|Tick|SetComponentTickEnabled true)
    (for _array_element (Utilities|Array|MakeArray "/Script/Paper2D.PaperFlipbookComponent" "/Script/Paper2D.PaperSpriteComponent")
      (CallFunction|SortPriority _array_element))))

(event EventTick
  (params (DeltaSeconds :type Float%20%28single-precision%29))
  (for _array_element (Utilities|Array|MakeArray "/Script/Paper2D.PaperFlipbookComponent" "/Script/Paper2D.PaperSpriteComponent")
    (CallFunction|SortPriority _array_element)))

(fn SortPriority
  (params (ComponentClass :type Actor%20Component%20Class%20Reference))
  (bind _returnvalue (Components|GetOwner))
  ;[1 0.7916 0.5059 0.3] Sorts the priority of the supported primitive components (Default Sprite Flipbooks and Sprite components) of the owning actor
  (for _array_element (Actor|GetComponentsByClass _returnvalue ComponentClass)
    (bind _asprimitive_component (Utilities|Casting|CastToPrimitiveComponent _array_element))
    (Rendering|SetTranslucentSortPriority _asprimitive_component (Math|Float|Truncate (.Y (Math|Vector|BreakVector (select (Variables|Default|GetbSortOnOwningActorLocation) (Transformation|GetActorLocation _returnvalue) (Transformation|GetWorldLocation _asprimitive_component))))))))