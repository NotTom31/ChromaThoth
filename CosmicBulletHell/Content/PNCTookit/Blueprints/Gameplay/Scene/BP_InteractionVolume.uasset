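; BP_InteractionVolume is a scene volume that registers itself with the interaction manager on Begin Play and references a list of assigned actors.
; Its construction script creates the cube's dynamic material, unhides each assigned actor and adds an arrow pointing toward it.
; Debug mode shows the cube and tints it on overlap.
; An IsValidTimeout macro retries validity checks with short delays before timing out.
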(event OnComponentBeginOverlap(Cube)
  (params (OverlappedComponent :type Primitive%20Component%20Object%20Reference) (OtherActor :type Actor%20Object%20Reference) (OtherComp :type Primitive%20Component%20Object%20Reference) (OtherBodyIndex :type Integer) (bFromSweep :type Boolean) (SweepResult :type Hit%20Result%20Structure%20%28by%20ref%29))
  ;[1 0.6073 0.1674 0.3] Handle debug events (Display debug volume)
  (if (Variables|InteractionVolume|GetbDebugEnabled)
    (Rendering|Material|SetVectorParameterValue (Variables|Default|GetDynamicMaterialInstance) "Colour" "(R=1.000000,G=0.000000,B=0.052035,A=1.000000)" :!class /Script/Engine.MaterialInstanceDynamic)))

(event OnComponentEndOverlap(Cube)
  (params (OverlappedComponent :type Primitive%20Component%20Object%20Reference) (OtherActor :type Actor%20Object%20Reference) (OtherComp :type Primitive%20Component%20Object%20Reference) (OtherBodyIndex :type Integer))
  ;[1 0.6073 0.1674 0.3] Handle debug events (Display debug volume)
  (if (Variables|InteractionVolume|GetbDebugEnabled)
    (Rendering|Material|SetVectorParameterValue (Variables|Default|GetDynamicMaterialInstance) "Colour" "(R=1.000000,G=1.000000,B=1.000000,A=1.000000)" :!class /Script/Engine.MaterialInstanceDynamic)))

(event Custom|EnableDebug
  (params (bDebugEnabled :type Boolean))
  ;[1 0.6073 0.1674 0.3] Handle debug events (Display debug volume)
  (bind _output_get (Variables|InteractionVolume|SetbDebugEnabled bDebugEnabled))
  (if _output_get
    (Rendering|SetVisibility (Variables|Default|GetCube) true false)
    (Development|SetHiddeninGame (Variables|Default|GetCube) false false)
    (else
      (Rendering|SetVisibility (Variables|Default|GetCube) false false)
      (Development|SetHiddeninGame (Variables|Default|GetCube) true false))))

(event EventBeginPlay
  (bind _return (CallFunction|GetInteractionManager))
  ;[1 0.7555 0.3037 0.3] On Begin Play, add itself to the interaction manager
  (Utilities|IsValid _return
    (:Is%20Valid
      (Default|AddInteractionVolume _return self))))

(fn ConstructionScript
  (bind _assignedactorsref (Variables|InteractionVolume|GetAssignedActorsRef))
  (bind _returnvalue (Rendering|Material|CreateDynamicMaterialInstance (Variables|Default|GetCube) 0 "/Game/PNCTookit/PNCGame/Scenes/Shared/Materials/MI_InteractionVolume_Inst.MI_InteractionVolume_Inst" "None" :!class /Script/Engine.PrimitiveComponent))
  (Variables|Default|SetDynamicMaterialInstance _returnvalue)
  (if (>= (Utilities|Array|Length _assignedactorsref) 1)
    (for _array_element _assignedactorsref
      (Utilities|IsValid _array_element
        (:Is%20Valid
          (bind _returnvalue_2 (AddComponent|AddArrowComponent false))
          (Rendering|SetActorHiddenInGame _array_element false)
          (Transformation|SetWorldRotation _returnvalue_2 (Math|Rotator|FindLookatRotation (Transformation|GetActorLocation) (Transformation|GetActorLocation _array_element)) false false)
          (Transformation|SetWorldScale3D _returnvalue_2 "1.000000,1.000000,1.000000"))))))