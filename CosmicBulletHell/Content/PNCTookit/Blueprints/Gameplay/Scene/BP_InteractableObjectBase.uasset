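; Base Blueprint for interactable scene objects in the PNC toolkit, holding active and used state that child classes extend.
; BeginPlay runs Init, which calls the overridable LoadGameplayState to turn that state into visible gameplay state.
; Save and load functions pack or restore the flags, object data and any inventory component contents, and loading re-applies gameplay state.
; Inspection and use are override points; UseObject returns whether the object is active.
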(event EventBeginPlay
  ;[1 0.8991 0.2581 0.3] Initialize the interactable object when brought into the world.
  ;
  ; Note: If you use "Event Begin Play" in your child classes, be sure to also "Add Call to Parent" before doing anything else. If this isnt done, init wont be called and the object state may not load/ be setup properly and cause issues.
  (InteractableObject|Init))

(fn ConstructionScript)

(fn Init
  ;[0.2916 0.7981 1 0.3] Initialize
  (SaveandLoad|LoadGameplayState)
  (return))

(fn LoadGameplayState
  ;[1 0.7171 0.2353 0.3] Override this function in all interactable object child classes.
  ;
  ; While the "Init" function is used to load the "object" state,   this function will use the object state data (e.g. IsActive or IsUsed) to load the custom "gameplay" state of the object.
  ;
  ; For example, if one of the light objects in the scene had "IsUsed" set to 'true', this "Load Gameplay State" function will then set the light as visible in the scene.
  (return true))

(fn LoadInteractableObject
  (params (SaveData :type S%20Interactable%20Object%20State%20Structure))
  (Utilities|FlowControl|Sequence
    (:then_0
      ;[1 0.2598 0.2896 0.3] Is Active
      (Variables|ObjectState|SetbIsActive (Utilities|Struct|BreakSInteractableObjectState SaveData))
      ;[1 0.2598 0.2896 0.3] Is Used
      (Variables|ObjectState|SetbIsUsed (Utilities|Struct|BreakSInteractableObjectState SaveData))
      ;[0.2266 0.4129 1 0.3] If we have an Inventory component we want to load the current items.
      (bind _output_get (LocalVariables|SetInventoryComponentComponentToSave (Actor|GetComponentbyClass "/Game/PNCTookit/Blueprints/Components/BP_InventoryComponent.BP_InventoryComponent_C")))
      (Utilities|IsValid _output_get
        (:Is%20Valid
          (Default|SetInventory (LocalVariables|GetInventoryComponentComponentToSave) (Utilities|Struct|BreakSInteractableObjectState SaveData)))))
    (:then_1
      (SaveandLoad|LoadGameplayState)
      (return))))

(fn GetInteractableSaveData
  (Utilities|FlowControl|Sequence
    (:then_0
      ;[0.2266 0.4129 1 0.3] If we have an Inventory component we want to save the current items so we can load them back in later.
      (bind _output_get (LocalVariables|SetInventoryComponentComponentToSave (Actor|GetComponentbyClass "/Game/PNCTookit/Blueprints/Components/BP_InventoryComponent.BP_InventoryComponent_C")))
      (Utilities|IsValid _output_get
        (:Is%20Valid
          (LocalVariables|SetInventory (Default|GetInventory (LocalVariables|GetInventoryComponentComponentToSave))))))
    (:then_1
      (return (Utilities|Struct|MakeSInteractableObjectState (Variables|ObjectState|GetbIsActive) (Variables|ObjectState|GetbIsUsed) (LocalVariables|GetInventory) (LocalVariables|GetInteractableData))))))

(fn OnInspection
  (params (Inspector :type Controller%20Object%20Reference))
  ;[1 0.9411 0.3122 0.3] Override this in children classes to handle inspection dialogue/functionality
  (CallFunction|CustomPrint "Inspecting Actor.  Override \"On Inspection\" interface function in the child blueprint." "NewEnumerator3" false)
  (return false))

(fn UseObject
  (params (InteractingCharacter :type BP%20PNC%20Character%20Parent%20Object%20Reference))
  ;[1 0.5293 0.7243 0.3] Children should override this function but still call it to see whether or not the object is currently active.
  (return (Variables|ObjectState|GetbIsActive)))