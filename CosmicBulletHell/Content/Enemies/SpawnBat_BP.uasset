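; SpawnBat_BP is an enemy spawner that releases up to twenty bats over time in the level.
; On BeginPlay it gathers all Wall actors, then runs a DoN loop paced by random delays of a few seconds.
; Each pass spawns a scaled-down Bat_BP above a randomly picked wall, with a rotation computed from a wall location toward the BP_AIPlayer.
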(event EventBeginPlay
  (bind _outactors (Actor|GetAllActorsOfClass "/Game/GridMovement/Wall.Wall_C"))
  (Variables|Default|SetWallArray _outactors)
  (Utilities|FlowControl|DoN 20 :!label _label
    (:Exit
      (Utilities|FlowControl|Sequence
        (:then_0
          (bind _returnvalue (Actor|GetActorOfClass "/Game/GridMovement/BP_AIPlayer.BP_AIPlayer_C"))
          (Game|SpawnActorfromClass "/Game/Enemies/Bat_BP.Bat_BP_C" (Math|Transform|MakeTransform (+ "0.000000,0.000000,100.000000" (Transformation|GetActorLocation (Utilities|Array|Get(acopy) (Variables|Default|GetWallArray) (Math|Random|RandomInteger (Utilities|Array|Length (Variables|Default|GetWallArray)))))) (Math|Rotator|FindLookatRotation (Transformation|GetActorLocation (Utilities|Array|Get(acopy) (Variables|Default|GetWallArray) (Math|Random|RandomInteger (Utilities|Array|Length (Variables|Default|GetWallArray))))) (Transformation|GetActorLocation _returnvalue)) "0.250000,0.250000,0.250000") "Undefined" "MultiplyWithRoot" 0 0))
        (:then_1
          (Utilities|FlowControl|Delay (Math|Random|RandomFloatinRange 1.0 1e+01))
          (goto _label))))))

(event Collision|EventActorBeginOverlap
  (params (OtherActor :type Actor%20Object%20Reference)))

(event EventTick
  (params (DeltaSeconds :type Float%20%28single-precision%29)))

(fn ConstructionScript)