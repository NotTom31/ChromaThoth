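; Bat enemy that chases the player and dies on contact with a bullet or the player.
; Every tick it casts itself to Pawn and issues AI Move To toward player pawn 0's current location.
; Its sprite's overlap destroys both bat and Bullet, or prints "OW" and destroys only the bat on hitting BP_AIPlayer.
; An unconnected manual look-at and offset movement chain remains unused.
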(event OnComponentBeginOverlap(bat_enemy_Sprite)
  (params (OverlappedComponent :type Primitive%20Component%20Object%20Reference) (OtherActor :type Actor%20Object%20Reference) (OtherComp :type Primitive%20Component%20Object%20Reference) (OtherBodyIndex :type Integer) (bFromSweep :type Boolean) (SweepResult :type Hit%20Result%20Structure%20%28by%20ref%29))
  (bind _asbullet (Utilities|Casting|CastToBullet OtherActor)
    (:then
      (Actor|DestroyActor _asbullet)
      (Actor|DestroyActor))
    (:CastFailed
      (Utilities|Casting|CastToBP_AIPlayer OtherActor)
      (Development|PrintString "OW")
      (Actor|DestroyActor))))

(event EventBeginPlay)

(event Collision|EventActorBeginOverlap
  (params (OtherActor :type Actor%20Object%20Reference)))

(event EventTick
  (params (DeltaSeconds :type Float%20%28single-precision%29))
  (bind _aspawn (Utilities|Casting|CastToPawn self))
  (AI|AIMoveTo _aspawn (Transformation|GetActorLocation (Game|Player|GetPlayerPawn 0)) 0 5.0 false))

(fn ConstructionScript)