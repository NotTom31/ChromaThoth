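; AI-driven pawn in the GridMovement folder that chases the player.
; Every Tick issues an AI MoveTo toward the location of player pawn 0, with zero acceptance radius.
; Set Coord stores that pawn's truncated world X and Y in TileToMoveTo and prints a debug string, but the chase does not use it.
; Get Coord is an empty stub.
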(event EventBeginPlay)

(event EventTick
  (params (DeltaSeconds :type Float%20%28single-precision%29))
  (AI|AIMoveTo self (Transformation|GetActorLocation (Game|Player|GetPlayerPawn 0)) 0 0.0 false))

(fn ConstructionScript)

(fn GetCoord)

(fn SetCoord
  (bind _returnvalue (Game|Player|GetPlayerPawn 0))
  (bind _returnvalue_2 (Transformation|GetActorLocation _returnvalue))
  (Variables|Default|SetTile%20to%20Move%20To (Utilities|Struct|MakeCoord (Math|Float|Truncate (.x _returnvalue_2)) (Math|Float|Truncate (.y _returnvalue_2))))
  (Development|PrintString "Set coord"))